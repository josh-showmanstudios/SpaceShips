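; Main game mode that tracks player controllers and handles spawning of player cameras and character pawns.
; InitNewPc adds unique entries to the PCs list; its loop over that list has no active body.
; SpawnCam destroys the controller's current pawn, then spawns and possesses a PPlayerCam at the first PlayerStart found.
; PawnSpawn creates and returns an ACharacterPawn a fixed distance in front of a given camera.
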(event Custom|InitNewPc
  (params (NewItem :type PC-Main%20Object%20Reference%20%28by%20ref%29))
  (bind _pcs (Variables|Default|GetPCs))
  (Utilities|Array|AddUnique _pcs NewItem)
  (for _array_element _pcs
    _))

(event Custom|SpawnCam
  (params (PlayerController :type Controller%20Object%20Reference))
  (bind _returnvalue (Pawn|GetControlledPawn PlayerController))
  (bind _outactors (Actor|GetAllActorsOfClass "/Script/Engine.PlayerStart"))
  (Utilities|IsValid _returnvalue
    (:Is%20Valid
      (Actor|DestroyActor _returnvalue))
    (:Is%20Not%20Valid
      _))
  (bind _returnvalue_2 (Game|SpawnActorfromClass "/Game/Blueprints/Pawns/P-PlayerCam.P-PlayerCam_C" (Transformation|GetActorTransform (Utilities|Array|Get(acopy) _outactors)) "AdjustIfPossibleButAlwaysSpawn" "MultiplyWithRoot" 0 0))
  (Pawn|Possess PlayerController _returnvalue_2))

(event EventBeginPlay)

(event EventTick
  (params (DeltaSeconds :type Float%20%28single-precision%29)))

(fn ConstructionScript)

(fn PawnSpawn
  (params (Cam :type Actor%20Object%20Reference))
  (bind _returnvalue (Transformation|GetActorTransform Cam))
  (bind _returnvalue_2 (Game|SpawnActorfromClass "/Game/Blueprints/Actors/A-CharacterPawn.A-CharacterPawn_C" (Math|Transform|MakeTransform (+ (.location _returnvalue) (* (Transformation|GetActorForwardVector Cam) 5e+02)) (.rotation _returnvalue) (.scale _returnvalue)) "AdjustIfPossibleButAlwaysSpawn" "MultiplyWithRoot" 0 0))
  (return _returnvalue_2))