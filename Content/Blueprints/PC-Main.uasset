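; Player controller that sets up each player's camera pawn and main HUD, and lets them spawn a pawn.
; On local BeginPlay it registers with GM-Main, requests a camera, then retries until it controls P-PlayerCam before adding the widget.
; P calls the camera's SpawnPawn only once.
; Paired Server/Cast-style events relay init and spawn requests to the game mode, storing the spawned pawn in RepCharPawn.
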(event Custom|SpawnCam
  (CallFunction|CastSpawnCam))

(event Custom|CastInitPC
  (bind _asgm_main (Utilities|Casting|CastToGM-Main (Game|GetGameMode)))
  (Default|InitNewPc _asgm_main self))

(event Custom|CastSpawnCam
  (bind _asgm_main (Utilities|Casting|CastToGM-Main (Game|GetGameMode)))
  (Default|SpawnCam _asgm_main self))

(event Custom|CastSpawnPawn
  (bind _asgm_main (Utilities|Casting|CastToGM-Main (Game|GetGameMode)))
  (bind _pawn (Default|PawnSpawn _asgm_main (Pawn|GetControlledPawn)))
  (Variables|Default|SetRepCharPawn _pawn))

(event Custom|SpawnPawn
  (params (PC :type PC-Main%20Object%20Reference))
  (CallFunction|CastSpawnPawn))

(event Custom|ServerInitPc
  (CallFunction|CastInitPC))

(event Custom|ServerSetCam
  (params (Cam :type P-Player%20Cam%20Object%20Reference))
  (CallFunction|CastSetCam Cam))

(event Custom|CastSetCam
  (params (Cam :type P-Player%20Cam%20Object%20Reference))
  (Variables|Default|SetCam Cam))

(event EventTick
  (params (DeltaSeconds :type Float%20%28single-precision%29)))

(event EventBeginPlay
  (Variables|Default|SetcanSpawn true)
  (if (Pawn|IsLocalController)
    (CallFunction|ServerInitPc)
    (Utilities|FlowControl|Delay 0.2)
    (CallFunction|SpawnCam)
    (bind _asp_player_cam (Utilities|Casting|CastToP-PlayerCam (Pawn|GetControlledPawn) :!label _label)
      (:then
        (bind _output_get (Variables|Default|SetCam _asp_player_cam))
        (CallFunction|ServerSetCam _output_get)
        (bind _returnvalue (UserInterface|CreateWidget "/Game/Blueprints/UI/W-MainGame.W-MainGame_C" self))
        (UserInterface|Viewport|AddtoViewport _returnvalue 0))
      (:CastFailed
        (Utilities|FlowControl|Delay 1.0)
        (goto _label)))))

(event Input|KeyboardEvents|P
  (params (Key :type Key%20Structure :default "None"))
  (:Pressed
    (Utilities|IsValid (Variables|Default|GetCam)
      (:Is%20Valid
        (if (Variables|Default|GetcanSpawn)
          (Variables|Default|SetcanSpawn false)
          (Default|SpawnPawn (Variables|Default|GetCam))))
      (:Is%20Not%20Valid
        (Development|PrintString "CantSpawnPawn")))))

(fn ConstructionScript)

(fn OnRepCharPawn)