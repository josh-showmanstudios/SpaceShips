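; Player camera pawn that spawns a separate character, attaches to its camera point and relays the player's input to it.
; Routes movement through one of three swappable components: zero-G, ship plane gravity or planet sphere gravity.
; A sphere trace finds gravity areas to attach to, and ship gravity allows driving by swapping input mapping contexts.
; Server-to-Cast event pairs replicate spawning, attach/detach and ship controls, with attach/detach skipping the local instance.
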(event Custom|OnServerAttachSphere
  (params (Parent :type Scene%20Component%20Object%20Reference))
  ;[0.15 0.15 0.15 0.5] Gravity attach/detach
  (CallFunction|CastAttachSphere Parent))

(event Custom|OnServerDetach
  (params (Pawn :type Actor%20Object%20Reference%20%28by%20ref%29))
  ;[0.15 0.15 0.15 0.5] Gravity attach/detach
  (CallFunction|CastDetach))

(event Custom|CheckHasChar
  (bind _pawnactor (Variables|Default|GetPawnActor))
  (bind _campos (Variables|/Game/Blueprints/Actors/A-CharacterPawn.A-CharacterPawn_C|GetCamPos _pawnactor))
  (bind _returnvalue (Transformation|GetWorldTransform _campos))
  (Utilities|IsValid (Variables|Default|GetPawnActor)
    (:Is%20Valid
      (Transformation|AttachComponentToComponent _campos "None" "KeepWorld" "KeepWorld" "KeepWorld" false)
      (Transformation|SetActorTransform (Math|Transform|MakeTransform (.location _returnvalue) (.rotation _returnvalue) "1.000000,1.000000,1.000000"))
      (Variables|Components|SetPawnMovementControl (Variables|Default|GetAC-NoGravControl))
      (Components|Tick|SetComponentTickEnabled (Variables|Default|GetAC-PlaneGravControl) false)
      (Components|Tick|SetComponentTickEnabled (Variables|Default|GetAC-NoGravControl) true)
      (Input|AddMappingContext (PlayerController|LocalPlayerSubsystems|GetEnhancedInputLocalPlayerSubsystem (Game|GetPlayerController 0)) "/Game/Input/IMC-Pawn.IMC-Pawn" 0 "(bIgnoreAllPressedKeysUntilRelease=True,bForceImmediately=False,bNotifyUserSettings=False)"))
    (:Is%20Not%20Valid
      (Utilities|FlowControl|Delay 0.1)
      (CallFunction|CheckHasChar))))

(event Custom|SpawnPawn
  (CallFunction|ServerSpawnPawn (Transformation|GetActorLocation) (Transformation|GetActorRotation))
  (Utilities|FlowControl|Delay 0.2)
  (CallFunction|CheckHasChar))

(event Custom|ServerShipThrust
  (params (Target :type A-Base%20Ship%20Object%20Reference) (ip :type Float%20%28double-precision%29))
  ;[0.15 0.15 0.15 0.5] Ship driving input
  (CallFunction|CastShipThust Target ip))

(event Custom|CastShipThust
  (params (Target :type A-Base%20Ship%20Object%20Reference) (ip :type Float%20%28double-precision%29))
  ;[0.15 0.15 0.15 0.5] Ship driving input
  (Default|ThrustCall Target ip))

(event Custom|CastShipRoll
  (params (Target :type A-Base%20Ship%20Object%20Reference) (ip :type Float%20%28double-precision%29))
  ;[0.15 0.15 0.15 0.5] Ship driving input
  (Default|RollCall Target ip))

(event Custom|CastShipPull
  (params (Target :type A-Base%20Ship%20Object%20Reference) (ip :type Float%20%28double-precision%29))
  ;[0.15 0.15 0.15 0.5] Ship driving input
  (Default|PullCall Target ip))

(event Custom|CastShipTurn
  (params (Target :type A-Base%20Ship%20Object%20Reference) (ip :type Float%20%28double-precision%29))
  ;[0.15 0.15 0.15 0.5] Ship driving input
  (Default|TurnCall Target ip))

(event Custom|ServerShipRoll
  (params (Target :type A-Base%20Ship%20Object%20Reference) (ip :type Float%20%28double-precision%29))
  ;[0.15 0.15 0.15 0.5] Ship driving input
  (CallFunction|CastShipRoll Target ip))

(event Custom|CastDetach
  (bind _pawnactor (Variables|Default|GetPawnActor))
  ;[0.15 0.15 0.15 0.5] Gravity attach/detach
  (if (not (Variables|Default|GetIsLocal))
    (Transformation|DetachFromActor (Variables|Default|GetPawnActor) "KeepWorld" "KeepWorld" "KeepWorld")
    (Components|Tick|SetComponentTickEnabled (Variables|Default|GetAC-PlaneGravControl) false)
    (Components|Tick|SetComponentTickEnabled (Variables|Default|GetAC-NoGravControl) true)
    (Variables|/Game/Blueprints/Actors/A-CharacterPawn.A-CharacterPawn_C|SetcurXSpeed _pawnactor 0.0)
    (Variables|/Game/Blueprints/Actors/A-CharacterPawn.A-CharacterPawn_C|SetcurYSpeed _pawnactor 0.0)
    (Variables|/Game/Blueprints/Actors/A-CharacterPawn.A-CharacterPawn_C|SetisInAir _pawnactor true)))

(event Custom|ServerShipPull
  (params (Target :type A-Base%20Ship%20Object%20Reference) (ip :type Float%20%28double-precision%29))
  ;[0.15 0.15 0.15 0.5] Ship driving input
  (CallFunction|CastShipPull Target ip))

(event Custom|PawnUse
  (bind _returnvalue (Game|GetPlayerController 0))
  (bind _returnvalue_2 (Game|GetPlayerController 0))
  (bind _returnvalue_3 (PlayerController|LocalPlayerSubsystems|GetEnhancedInputLocalPlayerSubsystem _returnvalue))
  (bind _returnvalue_4 (PlayerController|LocalPlayerSubsystems|GetEnhancedInputLocalPlayerSubsystem _returnvalue_2))
  ;[0.15 0.15 0.15 0.5] Use button
  (if (Variables|Default|GetisGrav)
    (if (Variables|/Game/Blueprints/Actors/A-CharacterPawn.A-CharacterPawn_C|GetisDrive (Variables|Default|GetPawnActor))
      (Variables|/Game/Blueprints/Actors/A-CharacterPawn.A-CharacterPawn_C|SetisDrive (Variables|Default|GetPawnActor) false)
      (Input|AddMappingContext _returnvalue_3 "/Game/Input/IMC-Pawn.IMC-Pawn" 0 "(bIgnoreAllPressedKeysUntilRelease=True,bForceImmediately=False,bNotifyUserSettings=False)")
      (Input|RemoveMappingContext _returnvalue_3 "/Game/Input/IMC-Ship.IMC-Ship" "(bIgnoreAllPressedKeysUntilRelease=True,bForceImmediately=False,bNotifyUserSettings=False)")
      (CallFunction|OnServerShipHasDriver (Variables|Default|Getship) false)
      (elif (Variables|Default|GetcanDrive)
        (Variables|/Game/Blueprints/Actors/A-CharacterPawn.A-CharacterPawn_C|SetisDrive (Variables|Default|GetPawnActor) true)
        (Input|AddMappingContext _returnvalue_4 "/Game/Input/IMC-Ship.IMC-Ship" 0 "(bIgnoreAllPressedKeysUntilRelease=True,bForceImmediately=False,bNotifyUserSettings=False)")
        (Input|RemoveMappingContext _returnvalue_4 "/Game/Input/IMC-Pawn.IMC-Pawn" "(bIgnoreAllPressedKeysUntilRelease=True,bForceImmediately=False,bNotifyUserSettings=False)")
        (CallFunction|OnServerShipHasDriver (Variables|Default|Getship) true)))))

(event Custom|ServerShipTurn
  (params (Target :type A-Base%20Ship%20Object%20Reference) (ip :type Float%20%28double-precision%29))
  ;[0.15 0.15 0.15 0.5] Ship driving input
  (CallFunction|CastShipTurn Target ip))

(event Custom|AttachToSphereGrav
  (params (Grav :type A-Base%20Sphere%20Gravity%20Object%20Reference))
  (bind _ac_nogravcontrol (Variables|Default|GetAC-NoGravControl))
  ;[0.15 0.15 0.15 0.5] Gravity attach/detach
  (Components|Tick|SetComponentTickEnabled (Variables|Default|GetAC-NoGravControl) false)
  (Variables|Default|SetisGrav true)
  (bind _output_get (Variables|Default|Setplanet Grav))
  (Transformation|AttachComponentToComponent (Variables|Default|GetPawnActor) (Variables|/Game/Blueprints/Actors/A-BaseSphereGravity.A-BaseSphereGravity_C|GetRoot _output_get) "None" "KeepWorld" "KeepWorld" "KeepWorld" false)
  (Variables|Components|SetPawnMovementControl (Variables|Default|GetAC-SphereGravControl))
  (CallFunction|OnServerAttachSphere (Variables|/Game/Blueprints/Actors/A-BaseSphereGravity.A-BaseSphereGravity_C|GetRoot (Variables|Default|Getplanet)))
  (Components|Tick|SetComponentTickEnabled (Variables|Default|GetAC-SphereGravControl) true)
  (Variables|/Game/Blueprints/Components/Player/AC-NoGravControl.AC-NoGravControl_C|SetSideInput _ac_nogravcontrol 0.0)
  (Variables|/Game/Blueprints/Components/Player/AC-NoGravControl.AC-NoGravControl_C|SetFwdInput _ac_nogravcontrol 0.0))

(event Custom|OnServerAttachPlane
  (params (Parent :type Scene%20Component%20Object%20Reference))
  ;[0.15 0.15 0.15 0.5] Gravity attach/detach
  (CallFunction|CastAttachPlane Parent))

(event Custom|CastAttachPlane
  (params (Parent :type Scene%20Component%20Object%20Reference))
  ;[0.15 0.15 0.15 0.5] Gravity attach/detach
  (if (not (Variables|Default|GetIsLocal))
    (Transformation|AttachComponentToComponent (Variables|Default|GetPawnActor) Parent "None" "KeepWorld" "KeepWorld" "KeepWorld" false)
    (Components|Tick|SetComponentTickEnabled (Variables|Default|GetAC-NoGravControl) false)
    (Components|Tick|SetComponentTickEnabled (Variables|Default|GetAC-PlaneGravControl) true)))

(event Custom|CastAttachSphere
  (params (Parent :type Scene%20Component%20Object%20Reference))
  ;[0.15 0.15 0.15 0.5] Gravity attach/detach
  (if (not (Variables|Default|GetIsLocal))
    (Transformation|AttachComponentToComponent (Variables|Default|GetPawnActor) Parent "None" "KeepWorld" "KeepWorld" "KeepWorld" false)
    (Components|Tick|SetComponentTickEnabled (Variables|Default|GetAC-NoGravControl) false)
    (Components|Tick|SetComponentTickEnabled (Variables|Default|GetAC-SphereGravControl) true)))

(event Custom|PawnActivateGravity
  ;[0.15 0.15 0.15 0.5] Gravity attach/detach
  (if (Variables|Default|GetisGrav)
    (CallFunction|DetachfromGravity)
    (Development|PrintString "detach")
    (else
      (CallFunction|CheckifGravity)
      (Development|PrintString "attach"))))

(event Custom|CastSpawnPawn
  (params (Spawn%20Transform%20Location :type Vector) (Spawn%20Transform%20Rotation :type Rotator))
  (bind _returnvalue (Game|SpawnActorfromClass "/Game/Blueprints/Actors/A-CharacterPawn.A-CharacterPawn_C" (Math|Transform|MakeTransform Spawn%20Transform%20Location Spawn%20Transform%20Rotation "1.000000,1.000000,1.000000") "AdjustIfPossibleButAlwaysSpawn" "MultiplyWithRoot" 0 0))
  (bind _output_get (Variables|Default|SetPawnActor _returnvalue))
  (Components|Tick|SetComponentTickEnabled (Variables|Default|GetAC-NoGravControl) true)
  (Development|PrintString (Utilities|String|Append "CHAR CREATED: " (Utilities|GetDisplayName _output_get))))

(event Custom|AttachToShipGravity
  (params (ship :type A-Base%20Ship%20Object%20Reference))
  (bind _pawnactor (Variables|Default|GetPawnActor))
  (bind _ac_nogravcontrol (Variables|Default|GetAC-NoGravControl))
  (bind _rootcomponent (Variables|/Script/Engine.Actor|GetRootComponent _pawnactor))
  ;[0.15 0.15 0.15 0.5] Gravity attach/detach
  (Components|Tick|SetComponentTickEnabled (Variables|Default|GetAC-NoGravControl) false)
  (Variables|Default|SetisGrav true)
  (bind _output_get (Variables|Default|SetShip ship))
  (Transformation|AttachComponentToComponent (Variables|Default|GetPawnActor) (Variables|/Game/Blueprints/Actors/A-BaseShip.A-BaseShip_C|GetRoot _output_get) "None" "KeepWorld" "KeepWorld" "KeepWorld" false)
  (Variables|Components|SetPawnMovementControl (Variables|Default|GetAC-PlaneGravControl))
  (CallFunction|OnServerAttachPlane (Variables|/Game/Blueprints/Actors/A-BaseShip.A-BaseShip_C|GetRoot (Variables|Default|GetShip)))
  (Components|Tick|SetComponentTickEnabled (Variables|Default|GetAC-PlaneGravControl) true)
  (Variables|/Game/Blueprints/Components/Player/AC-NoGravControl.AC-NoGravControl_C|SetSideInput _ac_nogravcontrol 0.0)
  (Variables|/Game/Blueprints/Components/Player/AC-NoGravControl.AC-NoGravControl_C|SetFwdInput _ac_nogravcontrol 0.0)
  (Transformation|SetRelativeRotation _rootcomponent (Math|Interpolation|RInterpTo (Variables|/Script/Engine.SceneComponent|GetRelativeRotation _rootcomponent) (Math|Rotator|MakeRotator 0.0 0.0 (.yaw (Variables|/Script/Engine.SceneComponent|GetRelativeRotation _rootcomponent))) 1.0 2.0) false false))

(event Custom|ServerSpawnPawn
  (params (Spawn%20Transform%20Location :type Vector) (Spawn%20Transform%20Rotation :type Rotator))
  (CallFunction|CastSpawnPawn Spawn%20Transform%20Location Spawn%20Transform%20Rotation))

(event Custom|DetachFromGravity
  (bind _ac_planegravcontrol (Variables|Default|GetAC-PlaneGravControl))
  (bind _pawnactor (Variables|Default|GetPawnActor))
  (bind _ac_spheregravcontrol (Variables|Default|GetAC-SphereGravControl))
  (bind _pawnactor_2 (Variables|Default|GetPawnActor))
  ;[0.15 0.15 0.15 0.5] Gravity attach/detach
  (Variables|/Game/Blueprints/Components/Player/AC-PlaneGravControl.AC-PlaneGravControl_C|SetxIp _ac_planegravcontrol 0.0)
  (Variables|/Game/Blueprints/Components/Player/AC-PlaneGravControl.AC-PlaneGravControl_C|SetyIp _ac_planegravcontrol 0.0)
  (Variables|/Game/Blueprints/Components/Player/AC-PlaneGravControl.AC-PlaneGravControl_C|SetjumpIp _ac_planegravcontrol 0.0)
  (Variables|/Game/Blueprints/Components/Player/AC-SphereGravControl.AC-SphereGravControl_C|SetxIp _ac_spheregravcontrol 0.0)
  (Variables|/Game/Blueprints/Components/Player/AC-SphereGravControl.AC-SphereGravControl_C|SetyIp _ac_spheregravcontrol 0.0)
  (Variables|/Game/Blueprints/Components/Player/AC-SphereGravControl.AC-SphereGravControl_C|SetjumpIp _ac_spheregravcontrol 0.0)
  (Components|Tick|SetComponentTickEnabled _ac_planegravcontrol false)
  (Variables|Default|SetisGrav false)
  (Variables|Default|SetcanDrive false)
  (Transformation|DetachFromActor (Variables|Default|GetPawnActor) "KeepWorld" "KeepWorld" "KeepWorld")
  (Variables|Components|SetPawnMovementControl (Variables|Default|GetAC-NoGravControl))
  (Transformation|SetActorRotation _pawnactor (Math|Interpolation|RInterpTo (Transformation|GetActorRotation _pawnactor) (Transformation|GetWorldRotation (Variables|Default|GetCamera)) 1.0 3.0))
  (Transformation|SetRelativeRotation (Variables|/Game/Blueprints/Actors/A-CharacterPawn.A-CharacterPawn_C|GetCameraRoot (Variables|Default|GetPawnActor)) (Math|Rotator|MakeRotator 0.0 0.0 0.0) false false)
  (CallFunction|OnServerDetach (Variables|Default|GetPawnActor))
  (Components|Tick|SetComponentTickEnabled (Variables|Default|GetAC-NoGravControl) true)
  (Variables|/Game/Blueprints/Actors/A-CharacterPawn.A-CharacterPawn_C|SetisInAir _pawnactor_2 true)
  (Variables|/Game/Blueprints/Actors/A-CharacterPawn.A-CharacterPawn_C|SetcurXSpeed _pawnactor_2 0.0)
  (Variables|/Game/Blueprints/Actors/A-CharacterPawn.A-CharacterPawn_C|SetcurYSpeed _pawnactor_2 0.0)
  (Variables|Default|SetShip 0)
  (Variables|Default|Setplanet 0))

(event Custom|OnServerShipHasDriver
  (params (Target :type A-Base%20Ship%20Object%20Reference) (hasDriver :type Boolean))
  ;[0.15 0.15 0.15 0.5] Use button
  (Default|SetHasDriver Target hasDriver))

(event Custom|CheckIfGravity
  (bind _pawnactor (Variables|Default|GetPawnActor))
  ;[0.15 0.15 0.15 0.5] Gravity attach/detach
  (bind (_outhit _returnvalue) (Collision|SphereTraceByChannel (Transformation|GetWorldLocation (Variables|/Game/Blueprints/Actors/A-CharacterPawn.A-CharacterPawn_C|GetBodyColTop _pawnactor)) (Transformation|GetWorldLocation (Variables|/Game/Blueprints/Actors/A-CharacterPawn.A-CharacterPawn_C|GetBodyColEnd _pawnactor)) 12.0 "TraceTypeQuery4" false 0 "None"))
  (if _returnvalue
    (if (Utilities|Enum|Equal(Enum) "GravArea" (Utilities|GetObjectName (.HitComponent (Collision|BreakHitResult _outhit)))) :!label _label
      (bind _asa_base_ship (Utilities|Casting|CastToA-BaseShip (Components|GetOwner (.HitComponent (Collision|BreakHitResult _outhit)))))
      (CallFunction|AttachtoShipGravity _asa_base_ship)
      (Utilities|Array|ForEachLoopwithBreak (Class|Actor|GetOverlappingComponents (Variables|Default|GetPawnActor)) :!label _label_2 ; enters at Break
        (:LoopBody
          (goto _label)))
      (elif (Utilities|Enum|Equal(Enum) "SphereGravArea" (Utilities|GetObjectName (.HitComponent (Collision|BreakHitResult _outhit))))
        (bind _asa_base_sphere_gravity (Utilities|Casting|CastToA-BaseSphereGravity (Components|GetOwner (.HitComponent (Collision|BreakHitResult _outhit)))))
        (CallFunction|AttachtoSphereGrav _asa_base_sphere_gravity)
        (goto _label_2 Break)))))

(event Input|EnhancedActionEvents|EnhancedInputActionIA_Use
  (params (ActionValue :type Boolean) (ElapsedSeconds :type Float%20%28double-precision%29) (TriggeredSeconds :type Float%20%28double-precision%29) (InputAction :type Input%20Action%20Object%20Reference :default "/Game/Input/Actions/Player/IA_Use.IA_Use"))
  ;[0.15 0.15 0.15 0.5] Pawn input
  (:Started
    (CallFunction|PawnUse)))

(event Input|EnhancedActionEvents|EnhancedInputActionIA_ShipThrust
  (params (ActionValue :type Float%20%28double-precision%29) (ElapsedSeconds :type Float%20%28double-precision%29) (TriggeredSeconds :type Float%20%28double-precision%29) (InputAction :type Input%20Action%20Object%20Reference :default "/Game/Input/Actions/Ship/IA_ShipThrust.IA_ShipThrust"))
  ;[0.15 0.15 0.15 0.5] Ship driving input
  (:Triggered
    (CallFunction|ServerShipThrust (Variables|Default|Getship) ActionValue :!label _label))
  (:Canceled
    (goto _label))
  (:Completed
    (goto _label)))

(event Input|EnhancedActionEvents|EnhancedInputActionIA_LookUp
  (params (ActionValue :type Float%20%28double-precision%29) (ElapsedSeconds :type Float%20%28double-precision%29) (TriggeredSeconds :type Float%20%28double-precision%29) (InputAction :type Input%20Action%20Object%20Reference :default "/Game/Input/Actions/Player/IA_LookUp.IA_LookUp"))
  ;[0.15 0.15 0.15 0.5] Pawn input
  (:Triggered
    (Default|LocalLookUp (Variables|Components|GetPawnMovementControl) ActionValue :!label _label))
  (:Canceled
    (goto _label))
  (:Completed
    (goto _label)))

(event Input|EnhancedActionEvents|EnhancedInputActionIA_LookRIght
  (params (ActionValue :type Float%20%28double-precision%29) (ElapsedSeconds :type Float%20%28double-precision%29) (TriggeredSeconds :type Float%20%28double-precision%29) (InputAction :type Input%20Action%20Object%20Reference :default "/Game/Input/Actions/Player/IA_LookRIght.IA_LookRIght"))
  ;[0.15 0.15 0.15 0.5] Pawn input
  (:Triggered
    (Default|LocalRotatePlayer (Variables|Components|GetPawnMovementControl) ActionValue :!label _label))
  (:Canceled
    (goto _label))
  (:Completed
    (goto _label)))

(event Input|EnhancedActionEvents|EnhancedInputActionIA_Jump
  (params (ActionValue :type Boolean) (ElapsedSeconds :type Float%20%28double-precision%29) (TriggeredSeconds :type Float%20%28double-precision%29) (InputAction :type Input%20Action%20Object%20Reference :default "/Game/Input/Actions/Player/IA_Jump.IA_Jump"))
  ;[0.15 0.15 0.15 0.5] Pawn input
  (:Started
    (Default|LocalJump (Variables|Components|GetPawnMovementControl) ActionValue)))

(event Input|EnhancedActionEvents|EnhancedInputActionIA_ActivateGravity
  (params (ActionValue :type Boolean) (ElapsedSeconds :type Float%20%28double-precision%29) (TriggeredSeconds :type Float%20%28double-precision%29) (InputAction :type Input%20Action%20Object%20Reference :default "/Game/Input/Actions/Player/IA_ActivateGravity.IA_ActivateGravity"))
  ;[0.15 0.15 0.15 0.5] Pawn input
  (:Started
    (CallFunction|PawnActivateGravity)))

(event Input|EnhancedActionEvents|EnhancedInputActionIA_Slide
  (params (ActionValue :type Float%20%28double-precision%29) (ElapsedSeconds :type Float%20%28double-precision%29) (TriggeredSeconds :type Float%20%28double-precision%29) (InputAction :type Input%20Action%20Object%20Reference :default "/Game/Input/Actions/Player/IA_Slide.IA_Slide"))
  ;[0.15 0.15 0.15 0.5] Pawn input
  (:Started
    (Default|LocalSlide (Variables|Components|GetPawnMovementControl) TriggeredSeconds)))

(event Input|EnhancedActionEvents|EnhancedInputActionIA_Crouch
  (params (ActionValue :type Boolean) (ElapsedSeconds :type Float%20%28double-precision%29) (TriggeredSeconds :type Float%20%28double-precision%29) (InputAction :type Input%20Action%20Object%20Reference :default "/Game/Input/Actions/Player/IA_Crouch.IA_Crouch"))
  ;[0.15 0.15 0.15 0.5] Pawn input
  (:Started
    (Default|LocalCrouch (Variables|Components|GetPawnMovementControl) TriggeredSeconds)))

(event Input|EnhancedActionEvents|EnhancedInputActionIA_ShipRoll
  (params (ActionValue :type Float%20%28double-precision%29) (ElapsedSeconds :type Float%20%28double-precision%29) (TriggeredSeconds :type Float%20%28double-precision%29) (InputAction :type Input%20Action%20Object%20Reference :default "/Game/Input/Actions/Ship/IA_ShipRoll.IA_ShipRoll"))
  ;[0.15 0.15 0.15 0.5] Ship driving input
  (:Triggered
    (CallFunction|ServerShipRoll (Variables|Default|Getship) ActionValue :!label _label))
  (:Canceled
    (goto _label))
  (:Completed
    (goto _label)))

(event Input|EnhancedActionEvents|EnhancedInputActionIA_MoveForward
  (params (ActionValue :type Float%20%28double-precision%29) (ElapsedSeconds :type Float%20%28double-precision%29) (TriggeredSeconds :type Float%20%28double-precision%29) (InputAction :type Input%20Action%20Object%20Reference :default "/Game/Input/Actions/Player/IA_MoveForward.IA_MoveForward"))
  ;[0.15 0.15 0.15 0.5] Pawn input
  (:Triggered
    (Default|LocalAddMovementX (Variables|Components|GetPawnMovementControl) ActionValue :!label _label))
  (:Canceled
    (goto _label))
  (:Completed
    (goto _label)))

(event Input|EnhancedActionEvents|EnhancedInputActionIA_ShipPull
  (params (ActionValue :type Float%20%28double-precision%29) (ElapsedSeconds :type Float%20%28double-precision%29) (TriggeredSeconds :type Float%20%28double-precision%29) (InputAction :type Input%20Action%20Object%20Reference :default "/Game/Input/Actions/Ship/IA_ShipPull.IA_ShipPull"))
  ;[0.15 0.15 0.15 0.5] Ship driving input
  (:Triggered
    (CallFunction|ServerShipPull (Variables|Default|Getship) ActionValue :!label _label))
  (:Canceled
    (goto _label))
  (:Completed
    (goto _label)))

(event Input|EnhancedActionEvents|EnhancedInputActionIA_ShipTurn
  (params (ActionValue :type Float%20%28double-precision%29) (ElapsedSeconds :type Float%20%28double-precision%29) (TriggeredSeconds :type Float%20%28double-precision%29) (InputAction :type Input%20Action%20Object%20Reference :default "/Game/Input/Actions/Ship/IA_ShipTurn.IA_ShipTurn"))
  ;[0.15 0.15 0.15 0.5] Ship driving input
  (:Triggered
    (CallFunction|ServerShipTurn (Variables|Default|Getship) ActionValue :!label _label))
  (:Canceled
    (goto _label))
  (:Completed
    (goto _label)))

(event Input|EnhancedActionEvents|EnhancedInputActionIA_MoveRIght
  (params (ActionValue :type Float%20%28double-precision%29) (ElapsedSeconds :type Float%20%28double-precision%29) (TriggeredSeconds :type Float%20%28double-precision%29) (InputAction :type Input%20Action%20Object%20Reference :default "/Game/Input/Actions/Player/IA_MoveRIght.IA_MoveRIght"))
  ;[0.15 0.15 0.15 0.5] Pawn input
  (:Triggered
    (Default|LocalAddMovementY (Variables|Components|GetPawnMovementControl) ActionValue :!label _label))
  (:Canceled
    (goto _label))
  (:Completed
    (goto _label)))

(event EventBeginPlay
  (bind _aspc_main (Utilities|Casting|CastToPC-Main (Game|GetPlayerController 0)))
  (Variables|Default|Setpc _aspc_main)
  (Utilities|FlowControl|Delay 1.0)
  (if (Pawn|IsLocallyControlled)
    (Variables|Default|SetIsLocal true)
    (else
      (Variables|Default|SetIsLocal false))))

(fn ConstructionScript)