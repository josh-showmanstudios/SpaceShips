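; Base ship pawn that flies with thrust, pitch, roll and turn inputs.
; Each tick, clamped inputs build decaying pulses that become a forward world offset and a combined axis-angle rotation around the ship's own axes.
; The server passes its location and rotation through CastLocRot; non-server instances run the same movement, then interpolate toward those values.
; An optional server-side demo applies automatic forward jumps and rotations every tick once its ten-second timer elapses.
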(event Custom|AddThrustPulse
  (CallFunction|PulsetoAdd (* (Math|Vector|GetForwardVector (Variables|Default|GetRoot)) (Variables|Default|GetThrustPower))))

(event Custom|DemoTurn
  (bind _root (Variables|Default|GetRoot))
  (bind _relativerotation (Variables|/Script/Engine.SceneComponent|GetRelativeRotation _root))
  (Transformation|SetRelativeRotation _root (Math|Interpolation|RInterpTo _relativerotation (Math|Rotator|CombineRotators _relativerotation (Math|Vector|RotatorfromAxisandAngle (Math|Vector|GetUpVector _relativerotation) 1.0)) 1.0 0.0) true false))

(event Custom|DemoPull
  (bind _root (Variables|Default|GetRoot))
  (bind _relativerotation (Variables|/Script/Engine.SceneComponent|GetRelativeRotation _root))
  (Transformation|SetRelativeRotation _root (Math|Interpolation|RInterpTo _relativerotation (Math|Rotator|CombineRotators _relativerotation (Math|Vector|RotatorfromAxisandAngle (Math|Vector|GetRightVector _relativerotation) 1.0)) 1.0 0.0) true false))

(event Custom|Demo
  (params (deltaTime :type Float%20%28double-precision%29))
  (if (Variables|Default|GetrunDemo)
    (bind _output_get (Variables|Default|SetdemoTimer (+ deltaTime (Variables|Default|GetdemoTimer))))
    (if (> _output_get 1e+01)
      (CallFunction|DemoFwd)
      (CallFunction|DemoPull)
      (CallFunction|DemoRoll)
      (CallFunction|DemoTurn))))

(event Custom|DemoFwd
  (CallFunction|PulsetoAdd (* (Math|Vector|GetForwardVector (Variables|Default|GetRoot)) 5e+03)))

(event Custom|ThrustCall
  (params (Ip :type Float%20%28double-precision%29))
  (Variables|Default|SetThrustInput (Math|Float|Clamp(Float) Ip)))

(event Custom|RollCalc
  (params (deltaTime :type Float%20%28double-precision%29))
  (bind _output_get (Variables|Default|SetRollPulse (+ (Variables|Default|GetRollPulse) (* (* deltaTime 3.0) (Variables|Default|GetRollInput)))))
  (if (> _output_get 0.0)
    (Variables|Default|SetRollPulse (Math|Float|Clamp(Float) (- _output_get deltaTime)))
    (Variables|Default|SetRollPower (* (Variables|Default|GetRollPulse) 0.5) :!label _label)
    (elif (< _output_get 0.0)
      (Variables|Default|SetRollPulse (Math|Float|Clamp(Float) (+ _output_get deltaTime) -1.0 0.0))
      (goto _label)
      (else
        (Variables|Default|SetRollPower 0.0)))))

(event Custom|TurnCall
  (params (Ip :type Float%20%28single-precision%29))
  (Variables|Default|SetTurnInput (Math|Float|Clamp(Float) Ip -1.0)))

(event Custom|RollCall
  (params (Ip :type Float%20%28single-precision%29))
  (Variables|Default|SetRollInput (Math|Float|Clamp(Float) Ip -1.0)))

(event Custom|ThrustCalc
  (params (deltaTime :type Float%20%28double-precision%29))
  (bind _output_get (Variables|Default|SetThrustPulse (Math|Float|Clamp(Float) (+ (- (Variables|Default|GetThrustPulse) deltaTime) (* (* deltaTime 3.0) (Variables|Default|GetThrustInput))))))
  (Variables|Default|SetThrustPower (* _output_get 1e+01)))

(event Custom|PullCall
  (params (Ip :type Float%20%28single-precision%29))
  (Variables|Default|SetPullInput (Math|Float|Clamp(Float) Ip -1.0)))

(event Custom|PullCalc
  (params (deltaTime :type Float%20%28double-precision%29))
  (bind _output_get (Variables|Default|SetPullPulse (+ (Variables|Default|GetPullPulse) (* (* deltaTime 1.5) (Variables|Default|GetPullInput)))))
  (if (> _output_get 0.0)
    (Variables|Default|SetPullPulse (Math|Float|Clamp(Float) (- _output_get deltaTime)))
    (Variables|Default|SetPullPower (* (Variables|Default|GetPullPulse) 0.5) :!label _label)
    (elif (< _output_get 0.0)
      (Variables|Default|SetPullPulse (Math|Float|Clamp(Float) (+ _output_get deltaTime) -1.0 0.0))
      (goto _label)
      (else
        (Variables|Default|SetPullPower 0.0)))))

(event Custom|TurnCalc
  (params (deltaTime :type Float%20%28double-precision%29))
  (bind _output_get (Variables|Default|SetTurnPulse (+ (Variables|Default|GetTurnPulse) (* (* deltaTime 3.0) (Variables|Default|GetTurnInput)))))
  (if (> _output_get 0.0)
    (Variables|Default|SetTurnPulse (Math|Float|Clamp(Float) (- _output_get deltaTime)))
    (Variables|Default|SetTurnPower (* (Variables|Default|GetTurnPulse) 0.5) :!label _label)
    (elif (< _output_get 0.0)
      (Variables|Default|SetTurnPulse (Math|Float|Clamp(Float) (+ _output_get deltaTime) -1.0 0.0))
      (goto _label)
      (else
        (Variables|Default|SetTurnPower 0.0)))))

(event Custom|PulseToAdd
  (params (DeltaLocation :type Vector))
  (Transformation|AddActorWorldOffset DeltaLocation))

(event Custom|SetHasDriver
  (params (hasDriver :type Boolean))
  (Variables|Default|SethasDriver hasDriver))

(event Custom|DemoRoll
  (bind _root (Variables|Default|GetRoot))
  (bind _relativerotation (Variables|/Script/Engine.SceneComponent|GetRelativeRotation _root))
  (Transformation|SetRelativeRotation _root (Math|Interpolation|RInterpTo _relativerotation (Math|Rotator|CombineRotators _relativerotation (Math|Vector|RotatorfromAxisandAngle (Math|Vector|GetForwardVector _relativerotation) 1.0)) 1.0 0.0) true false))

(event Custom|CastLocRot
  (params (castLoc :type Vector) (castRot :type Rotator))
  (Variables|Default|SetcastLoc castLoc)
  (Variables|Default|SetcastRot castRot))

(event Custom|AddTurnVel
  (bind _root (Variables|Default|GetRoot))
  (bind _relativerotation (Variables|/Script/Engine.SceneComponent|GetRelativeRotation _root))
  (Transformation|SetRelativeRotation _root (Math|Interpolation|RInterpTo _relativerotation (Math|Rotator|CombineRotators _relativerotation (Variables|Default|GetTurnVelocity)) 1.0 1.0) true false))

(event Custom|CalcTurnVel
  (bind _root (Variables|Default|GetRoot))
  (bind _relativerotation (Variables|/Script/Engine.SceneComponent|GetRelativeRotation _root))
  (Variables|Default|SetTurnVelocity (Math|Rotator|CombineRotators (Math|Rotator|CombineRotators (Math|Vector|RotatorfromAxisandAngle (Math|Vector|GetRightVector _relativerotation) (Variables|Default|GetPullPower)) (Math|Vector|RotatorfromAxisandAngle (Math|Vector|GetUpVector _relativerotation) (Variables|Default|GetTurnPower))) (Math|Vector|RotatorfromAxisandAngle (Math|Vector|GetForwardVector _relativerotation) (Variables|Default|GetRollPower)))))

(event EventBeginPlay
  (Variables|Default|SetdemoTimer 0.0)
  (if (not (Networking|IsServer))
    (Variables|Default|SetisServer false)
    (else
      (Variables|Default|SetisServer true))))

(event EventTick
  (params (DeltaSeconds :type Float%20%28single-precision%29))
  (bind _returnvalue (* DeltaSeconds 0.3))
  (CallFunction|ThrustCalc _returnvalue)
  (CallFunction|PullCalc _returnvalue)
  (CallFunction|RollCalc _returnvalue)
  (CallFunction|TurnCalc _returnvalue)
  (CallFunction|CalcTurnVel)
  (CallFunction|AddThrustPulse)
  (CallFunction|AddTurnVel)
  (if (Variables|Default|GetisServer)
    (CallFunction|CastLocRot (Transformation|GetWorldLocation (Variables|Transformation|GetRootComponent)) (Variables|/Script/Engine.SceneComponent|GetRelativeRotation (Variables|Default|GetRoot)))
    (CallFunction|Demo DeltaSeconds)
    (else
      (Transformation|SetWorldLocation (Variables|Transformation|GetRootComponent) (Math|Interpolation|VInterpTo (Transformation|GetWorldLocation (Variables|Transformation|GetRootComponent)) (Variables|Default|GetcastLoc) 1.0 1.0) false false)
      (Transformation|SetRelativeRotation (Variables|Default|GetRoot) (Math|Interpolation|RInterpTo (Variables|/Script/Engine.SceneComponent|GetRelativeRotation (Variables|Default|GetRoot)) (Variables|Default|GetcastRot) 1.0 1.0) false false))))

(fn ConstructionScript)