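; Actor component that moves its owner by swept local or world offsets, with move-and-slide variants for collisions.
; On a hit, the slide events project input onto the surface plane, then along the crease of two normals if blocked again, plus a reflection-based nudge.
; Local slides clamp out downward Z.
; IsSlopeSteep sphere-traces between the owner's floor-check points, comparing the normal to actor up; WallCheck is an empty stub with disconnected logic.
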(event Custom|WorldMove
  (params (deltaTime :type Float%20%28double-precision%29) (InputDir :type Vector))
  (Transformation|AddActorWorldOffset (Variables|Default|GetPawn%20Actor) (* deltaTime InputDir) true))

(event Custom|LocalMove
  (params (deltaTime :type Float%20%28double-precision%29) (InputDir :type Vector))
  (Transformation|AddActorLocalOffset (Variables|Default|GetPawn%20Actor) (* deltaTime InputDir) true false))

(event Custom|LocalMoveAndSlide
  (params (deltaTime :type Float%20%28double-precision%29) (InputDir :type Vector))
  (bind _returnvalue (* deltaTime InputDir))
  (bind _pawn_actor (Variables|Default|GetPawn%20Actor))
  (bind _returnvalue_2 (Transformation|GetActorTransform _pawn_actor))
  (bind _returnvalue_3 (Math|Transform|TransformDirection _returnvalue_2 InputDir))
  (bind _sweephitresult (Transformation|AddActorLocalOffset (Variables|Default|GetPawn%20Actor) (Math|Vector|MakeVector (.x _returnvalue) (.y _returnvalue) (Math|Float|Clamp(Float) (.z _returnvalue) -4.8e+03 4.8e+03)) true false))
  (if (.bBlockingHit (Collision|BreakHitResult _sweephitresult))
    (bind _sweephitresult_2 (Transformation|AddActorLocalOffset (Variables|Default|GetPawn%20Actor) (* (Math|Vector|MakeVector (.x (Math|Transform|InverseTransformDirection _returnvalue_2 (Math|Vector|ProjectVectorontoPlane _returnvalue_3 (.Normal (Collision|BreakHitResult _sweephitresult))))) (.y (Math|Transform|InverseTransformDirection _returnvalue_2 (Math|Vector|ProjectVectorontoPlane _returnvalue_3 (.Normal (Collision|BreakHitResult _sweephitresult))))) (Math|Float|Clamp(Float) (.z (Math|Transform|InverseTransformDirection _returnvalue_2 (Math|Vector|ProjectVectorontoPlane _returnvalue_3 (.Normal (Collision|BreakHitResult _sweephitresult))))) 0.0 4.8e+03)) deltaTime) true false))
    (if (.bBlockingHit (Collision|BreakHitResult _sweephitresult_2))
      (CallFunction|LocalMove deltaTime (Math|Vector|MakeVector (.x (Math|Transform|InverseTransformDirection _returnvalue_2 (Math|Vector|ProjectVectorontoVector _returnvalue_3 (Math|Vector|CrossProduct (.Normal (Collision|BreakHitResult _sweephitresult_2)) (.Normal (Collision|BreakHitResult _sweephitresult)))))) (.y (Math|Transform|InverseTransformDirection _returnvalue_2 (Math|Vector|ProjectVectorontoVector _returnvalue_3 (Math|Vector|CrossProduct (.Normal (Collision|BreakHitResult _sweephitresult_2)) (.Normal (Collision|BreakHitResult _sweephitresult)))))) (Math|Float|Clamp(Float) (.z (Math|Transform|InverseTransformDirection _returnvalue_2 (Math|Vector|ProjectVectorontoVector _returnvalue_3 (Math|Vector|CrossProduct (.Normal (Collision|BreakHitResult _sweephitresult_2)) (.Normal (Collision|BreakHitResult _sweephitresult)))))) 0.0 4.8e+03))))
    (CallFunction|LocalMove deltaTime (Math|Vector|MakeVector (* (.x (Math|Transform|InverseTransformDirection _returnvalue_2 (Math|Vector|GetReflectionVector (Math|Vector|GetUnitDirection(Vector) (.TraceStart (Collision|BreakHitResult _sweephitresult)) (.TraceEnd (Collision|BreakHitResult _sweephitresult))) (.Normal (Collision|BreakHitResult _sweephitresult))))) 1.0) (* (.y (Math|Transform|InverseTransformDirection _returnvalue_2 (Math|Vector|GetReflectionVector (Math|Vector|GetUnitDirection(Vector) (.TraceStart (Collision|BreakHitResult _sweephitresult)) (.TraceEnd (Collision|BreakHitResult _sweephitresult))) (.Normal (Collision|BreakHitResult _sweephitresult))))) 1.0) (* (Math|Float|Clamp(Float) (.z (Math|Transform|InverseTransformDirection _returnvalue_2 (Math|Vector|GetReflectionVector (Math|Vector|GetUnitDirection(Vector) (.TraceStart (Collision|BreakHitResult _sweephitresult)) (.TraceEnd (Collision|BreakHitResult _sweephitresult))) (.Normal (Collision|BreakHitResult _sweephitresult))))) 0.0 4.8e+03) 1.0)))))

(event Custom|WorldMoveAndSlide
  (params (deltaTime :type Float%20%28double-precision%29) (InputDir :type Vector))
  (bind _sweephitresult (Transformation|AddActorWorldOffset (Variables|Default|GetPawn%20Actor) (* deltaTime InputDir) true))
  (if (.bBlockingHit (Collision|BreakHitResult _sweephitresult))
    (bind _sweephitresult_2 (Transformation|AddActorLocalOffset (Variables|Default|GetPawn%20Actor) (* (Math|Vector|ProjectVectorontoPlane InputDir (.Normal (Collision|BreakHitResult _sweephitresult))) deltaTime) true false))
    (if (.bBlockingHit (Collision|BreakHitResult _sweephitresult_2))
      (CallFunction|WorldMove deltaTime (Math|Vector|ProjectVectorontoVector InputDir (Math|Vector|CrossProduct (.Normal (Collision|BreakHitResult _sweephitresult_2)) (.Normal (Collision|BreakHitResult _sweephitresult))))))
    (CallFunction|WorldMove deltaTime (Math|Vector|ProjectVectorontoVector InputDir (Math|Vector|GetReflectionVector (Math|Vector|GetUnitDirection(Vector) (.TraceStart (Collision|BreakHitResult _sweephitresult)) (.TraceEnd (Collision|BreakHitResult _sweephitresult))) (.Normal (Collision|BreakHitResult _sweephitresult)))))))

(event EventBeginPlay
  (Variables|Default|SetPawn%20Actor (Components|GetOwner)))

(fn IsSlopeSteep
  (bind _pawn_actor (Variables|Default|GetPawn%20Actor))
  (bind (_onfloorcheck _gravityonfloorcheck) (Class|BPI-ActorPawn|GetGravityFloorCheck(Message) _pawn_actor))
  (bind _outhit (Collision|SphereTraceByChannel (Transformation|GetWorldLocation _onfloorcheck) (Transformation|GetWorldLocation _gravityonfloorcheck) 9.0 "TraceTypeQuery1" false 0 "None"))
  (if (> (Class|KismetMathLibrary|DegAcos (Math|Vector|DotProduct (.Normal (Collision|BreakHitResult _outhit)) (Transformation|GetActorUpVector _pawn_actor))) 45.5)
    (return true)
    (else
      (return false))))

(fn WallCheck
  (params (InputDir :type Vector) (DeltaTime :type Float%20%28double-precision%29)))

(fn FuncRelMoveandSlide
  (params (HitNormal :type Vector) (RelInputInWorld :type Vector) (ActorTransform :type Transform) (DeltaTime :type Float%20%28double-precision%29))
  (bind _returnvalue (Math|Vector|ProjectVectorontoPlane RelInputInWorld HitNormal))
  (bind _returnvalue_2 (Math|Transform|InverseTransformDirection ActorTransform _returnvalue))
  (bind _returnvalue_3 (Math|Float|Clamp(Float) (.z _returnvalue_2) 0.0 4.8e+03))
  (CallFunction|LocalMove DeltaTime (Math|Vector|MakeVector (.x _returnvalue_2) (.y _returnvalue_2) _returnvalue_3))
  (for _index (range 1 10)
    (CallFunction|LocalMove DeltaTime (Math|Vector|MakeVector (* (.x _returnvalue_2) 0.1) (* (.y _returnvalue_2) 0.1) (* _returnvalue_3 0.1)))))