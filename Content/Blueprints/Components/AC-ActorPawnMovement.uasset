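; Actor component that moves its owning A-PlayerPawn with swept offsets, caching the pawn on BeginPlay.
; It exposes local, world and root-relative move events, each scaling input direction by speed and delta time.
; Their MoveAndSlide variants handle blocking hits by reflecting the trace direction off the hit normal, then making a second full-step world move toward the impact location plus that reflection.
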(event Custom|WorldMove
  (params (deltaTime :type Float%20%28double-precision%29) (InputDir :type Vector) (Speed :type Float%20%28single-precision%29))
  (Transformation|AddActorWorldOffset (Variables|Default|GetPawn%20Actor) (* deltaTime InputDir Speed) true))

(event Custom|LocalMove
  (params (deltaTime :type Float%20%28double-precision%29) (InputDir :type Vector) (Speed :type Float%20%28single-precision%29))
  (Transformation|AddActorLocalOffset (Variables|Default|GetPawn%20Actor) (* deltaTime InputDir Speed) true false))

(event Custom|RelativeMove
  (params (deltaTime :type Float%20%28double-precision%29) (InputDir :type Vector) (Speed :type Float%20%28double-precision%29))
  (Transformation|AddRelativeLocation (Variables|/Script/Engine.Actor|GetRootComponent (Variables|Default|GetPawn%20Actor)) (* deltaTime InputDir Speed) true false))

(event Custom|LocalMoveAndSlide
  (params (deltaTime :type Float%20%28double-precision%29) (InputDir :type Vector) (Speed :type Float%20%28single-precision%29))
  (bind _sweephitresult (Transformation|AddActorLocalOffset (Variables|Default|GetPawn%20Actor) (* deltaTime InputDir Speed) true false))
  (if (.bBlockingHit (Collision|BreakHitResult _sweephitresult))
    (CallFunction|WorldMove deltaTime (Math|Vector|GetUnitDirection(Vector) (Transformation|GetActorLocation (Variables|Default|GetPawn%20Actor)) (+ (.Location (Collision|BreakHitResult _sweephitresult)) (Math|Vector|GetReflectionVector (Math|Vector|GetUnitDirection(Vector) (.TraceStart (Collision|BreakHitResult _sweephitresult)) (.TraceEnd (Collision|BreakHitResult _sweephitresult))) (.Normal (Collision|BreakHitResult _sweephitresult))))) Speed)))

(event Custom|RelativeMoveAndSlide
  (params (deltaTime :type Float%20%28double-precision%29) (InputDir :type Vector) (Speed :type Float%20%28double-precision%29))
  (bind _sweephitresult (Transformation|AddRelativeLocation (Variables|/Script/Engine.Actor|GetRootComponent (Variables|Default|GetPawn%20Actor)) (* deltaTime InputDir Speed) true false))
  (if (.bBlockingHit (Collision|BreakHitResult _sweephitresult))
    (CallFunction|WorldMove deltaTime (Math|Vector|GetUnitDirection(Vector) (Transformation|GetActorLocation (Variables|Default|GetPawn%20Actor)) (+ (.Location (Collision|BreakHitResult _sweephitresult)) (Math|Vector|GetReflectionVector (Math|Vector|GetUnitDirection(Vector) (.TraceStart (Collision|BreakHitResult _sweephitresult)) (.TraceEnd (Collision|BreakHitResult _sweephitresult))) (.Normal (Collision|BreakHitResult _sweephitresult))))) Speed)))

(event Custom|WorldMoveAndSlide
  (params (deltaTime :type Float%20%28double-precision%29) (InputDir :type Vector) (Speed :type Float%20%28double-precision%29))
  (bind _sweephitresult (Transformation|AddActorWorldOffset (Variables|Default|GetPawn%20Actor) (* deltaTime InputDir Speed) true))
  (if (.bBlockingHit (Collision|BreakHitResult _sweephitresult))
    (CallFunction|WorldMove deltaTime (Math|Vector|GetUnitDirection(Vector) (Transformation|GetActorLocation (Variables|Default|GetPawn%20Actor)) (+ (.Location (Collision|BreakHitResult _sweephitresult)) (Math|Vector|GetReflectionVector (Math|Vector|GetUnitDirection(Vector) (.TraceStart (Collision|BreakHitResult _sweephitresult)) (.TraceEnd (Collision|BreakHitResult _sweephitresult))) (.Normal (Collision|BreakHitResult _sweephitresult))))) Speed)))

(event EventBeginPlay
  (bind _asa_player_pawn (Utilities|Casting|CastToA-PlayerPawn (Components|GetOwner)))
  (Variables|Default|SetPawn%20Actor _asa_player_pawn))