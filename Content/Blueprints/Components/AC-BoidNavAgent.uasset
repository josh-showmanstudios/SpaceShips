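; NPC pawn component that steers its owner toward the player camera actor (PPlayerCam) without a navmesh, despite its boid name using no flocking.
; When line of sight is blocked, it sphere-traces one yaw step per tick, plus a pitched probe, adopting the point nearest the target after each sweep.
; While the target has gravity, the pawn attaches to overlapped ship or planet gravity areas, levelling on ships; planet alignment is empty.
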(event Custom|SetTargetLoc
  (if (Utilities|IsValid (Variables|Default|GettargetActor))
    (Variables|Default|SettargetLoc (Transformation|GetActorLocation (Variables|Default|GettargetActor)))
    (else
      (bind _returnvalue (Actor|GetActorOfClass "/Game/Blueprints/Pawns/P-PlayerCam.P-PlayerCam_C"))
      (Variables|Default|SettargetActor _returnvalue))))

(event Custom|TraceVertical
  (bind _outhit (Collision|SphereTraceByChannel (Transformation|GetActorLocation (Variables|Default|GetNpcPawn)) (+ (* (Math|Vector|RotateVector "1.000000, 0, 0" (Math|Rotator|MakeRotator 0.0 (Math|Conversions|ToFloat(Integer) (* (Variables|Default|GetvertFlip) 45)) (* (Variables|Default|GetcurTrace) 3e+01))) (* (Variables|Default|GetscanDis) 0.25)) (Transformation|GetActorLocation (Variables|Default|GetNpcPawn))) 2e+01 "TraceTypeQuery2" false 0 "ForDuration" true "(R=1.000000,G=0.000000,B=0.000000,A=1.000000)" "(R=0.000000,G=1.000000,B=0.000000,A=1.000000)" 0.1))
  (if (.bBlockingHit (Collision|BreakHitResult _outhit))
    (if (< (Math|Float|Absolute(Float) (Math|Vector|VectorLength (- (+ (.ImpactPoint (Collision|BreakHitResult _outhit)) (* (.ImpactNormal (Collision|BreakHitResult _outhit)) 1.2e+02)) (Variables|Default|GettargetLoc)))) (Variables|Default|GetminTravel))
      (Variables|Default|SetminTravel (Math|Float|Absolute(Float) (Math|Vector|VectorLength (- (+ (.ImpactPoint (Collision|BreakHitResult _outhit)) (* (.ImpactNormal (Collision|BreakHitResult _outhit)) 1.2e+02)) (Variables|Default|GettargetLoc)))))
      (Variables|Default|SetnextMoveLoc (+ (.ImpactPoint (Collision|BreakHitResult _outhit)) (* (.ImpactNormal (Collision|BreakHitResult _outhit)) 1.2e+02))))
    (elif (< (Math|Float|Absolute(Float) (Math|Vector|VectorLength (- (.TraceEnd (Collision|BreakHitResult _outhit)) (Variables|Default|GettargetLoc)))) (Variables|Default|GetminTravel))
      (Variables|Default|SetminTravel (Math|Float|Absolute(Float) (Math|Vector|VectorLength (- (.TraceEnd (Collision|BreakHitResult _outhit)) (Variables|Default|GettargetLoc)))))
      (Variables|Default|SetnextMoveLoc (.TraceEnd (Collision|BreakHitResult _outhit))))))

(event Custom|SetGravity
  (bind _targetactor (Variables|Default|GettargetActor))
  (bind _targetactor_2 (Variables|Default|GettargetActor))
  (bind _npcpawn (Variables|Default|GetNpcPawn))
  (bind _targetactor_3 (Variables|Default|GettargetActor))
  (bind _base (Variables|/Game/Blueprints/Actors/A-CharacterPawn.A-CharacterPawn_C|GetBase _npcpawn))
  (if (Utilities|IsValid (Variables|Default|GettargetActor))
    (if (Variables|/Game/Blueprints/Pawns/P-PlayerCam.P-PlayerCam_C|GetisGrav _targetactor_2)
      (if (Utilities|IsValid (Variables|/Game/Blueprints/Pawns/P-PlayerCam.P-PlayerCam_C|GetShip _targetactor_2))
        (if (Class|PrimitiveComponent|IsOverlappingComponent _base (Variables|/Game/Blueprints/Actors/A-BaseShip.A-BaseShip_C|GetGravArea (Variables|/Game/Blueprints/Pawns/P-PlayerCam.P-PlayerCam_C|GetShip _targetactor_3)))
          (Variables|Default|SetisGrav true)
          (Transformation|AttachComponentToComponent (Variables|Default|GetNpcPawn) (Variables|/Game/Blueprints/Actors/A-BaseShip.A-BaseShip_C|GetRoot (Variables|/Game/Blueprints/Pawns/P-PlayerCam.P-PlayerCam_C|GetShip _targetactor)) "None" "KeepWorld" "KeepWorld" "KeepWorld" false)
          (Variables|Default|SetisShip true)
          (else
            (Development|PrintString "TEST3")
            (Variables|Default|SetisGrav false :!label _label)
            (Transformation|DetachFromActor (Variables|Default|GetNpcPawn) "KeepWorld" "KeepWorld" "KeepWorld")
            (Variables|Default|SetisShip false)
            (Variables|Default|SetisPlanet false)))
        (elif (Utilities|IsValid (Variables|/Game/Blueprints/Pawns/P-PlayerCam.P-PlayerCam_C|Getplanet _targetactor_2))
          (if (Class|PrimitiveComponent|IsOverlappingComponent _base (Variables|/Game/Blueprints/Actors/A-BaseSphereGravity.A-BaseSphereGravity_C|GetSphereGravArea (Variables|/Game/Blueprints/Pawns/P-PlayerCam.P-PlayerCam_C|Getplanet _targetactor_3)))
            (Variables|Default|SetisGrav true)
            (Transformation|AttachComponentToComponent (Variables|Default|GetNpcPawn) (Variables|/Game/Blueprints/Actors/A-BaseSphereGravity.A-BaseSphereGravity_C|GetRoot (Variables|/Game/Blueprints/Pawns/P-PlayerCam.P-PlayerCam_C|Getplanet _targetactor)) "None" "KeepWorld" "KeepWorld" "KeepWorld" false)
            (Variables|Default|SetisPlanet true)
            (else
              (goto _label)))))
      (elif (Variables|Default|GetisGrav)
        (goto _label)))))

(event Custom|AddGrav
  (bind _npcpawn (Variables|Default|GetNpcPawn))
  (bind _rootcomponent (Variables|/Script/Engine.Actor|GetRootComponent _npcpawn))
  (if (Utilities|IsValid (Variables|Default|GettargetActor))
    (if (Variables|Default|GetisGrav)
      (if (Variables|Default|GetisShip)
        (Transformation|SetRelativeRotation _rootcomponent (Math|Rotator|MakeRotator 0.0 0.0 (.yaw (Variables|/Script/Engine.SceneComponent|GetRelativeRotation _rootcomponent))) false false)
        (Development|PrintString "WHAT")
        (elif (Variables|Default|GetisPlanet)
          _)))))

(event Custom|FindClosestPoint
  (bind _targetactor (Variables|Default|GettargetActor))
  (bind _actorstoignore (Variables|Default|GetActorsToIgnore))
  (Variables|Default|SetscanDis (Math|Float|Absolute(Float) (Math|Vector|VectorLength (- (Transformation|GetActorLocation (Variables|Default|GetNpcPawn)) (Variables|Default|GettargetLoc)))))
  (bind _outactors (Actor|GetAllActorsOfClass "/Game/Blueprints/Actors/A-NpcCharacterPawn.A-NpcCharacterPawn_C"))
  (Utilities|Set|AddItems _actorstoignore _outactors)
  (Utilities|Set|AddItems _actorstoignore (Utilities|Array|MakeArray _targetactor (Variables|/Game/Blueprints/Pawns/P-PlayerCam.P-PlayerCam_C|GetPawnActor _targetactor) 0))
  (bind _result (Utilities|Set|ToArray _actorstoignore))
  (bind _outhit (Collision|SphereTraceByChannel (Transformation|GetActorLocation (Variables|Default|GetNpcPawn)) (Variables|Default|GettargetLoc) 2e+01 "TraceTypeQuery2" false _result "None" true "(R=1.000000,G=0.000000,B=0.000000,A=1.000000)" "(R=0.000000,G=1.000000,B=0.000000,A=1.000000)" 0.1))
  (if (.bBlockingHit (Collision|BreakHitResult _outhit))
    (bind _outhit_2 (Collision|SphereTraceByChannel (Transformation|GetActorLocation (Variables|Default|GetNpcPawn)) (+ (* (Math|Vector|RotateVector "1.000000, 0, 0" (Math|Rotator|MakeRotator 0.0 0.0 (* (Variables|Default|GetcurTrace) 3e+01))) (Variables|Default|GetscanDis)) (Transformation|GetActorLocation (Variables|Default|GetNpcPawn))) 2e+01 "TraceTypeQuery2" false 0 "ForDuration" true "(R=1.000000,G=0.000000,B=0.000000,A=1.000000)" "(R=0.000000,G=1.000000,B=0.000000,A=1.000000)" 0.1))
    (if (.bBlockingHit (Collision|BreakHitResult _outhit_2))
      (if (< (Math|Float|Absolute(Float) (Math|Vector|VectorLength (- (+ (.ImpactPoint (Collision|BreakHitResult _outhit_2)) (* (.ImpactNormal (Collision|BreakHitResult _outhit_2)) 1.2e+02)) (Variables|Default|GettargetLoc)))) (Variables|Default|GetminTravel))
        (Variables|Default|SetminTravel (Math|Float|Absolute(Float) (Math|Vector|VectorLength (- (+ (.ImpactPoint (Collision|BreakHitResult _outhit_2)) (* (.ImpactNormal (Collision|BreakHitResult _outhit_2)) 1.2e+02)) (Variables|Default|GettargetLoc)))))
        (Variables|Default|SetnextMoveLoc (+ (.ImpactPoint (Collision|BreakHitResult _outhit_2)) (* (.ImpactNormal (Collision|BreakHitResult _outhit_2)) 1.2e+02))))
      (elif (< (Math|Float|Absolute(Float) (Math|Vector|VectorLength (- (.TraceEnd (Collision|BreakHitResult _outhit_2)) (Variables|Default|GettargetLoc)))) (Variables|Default|GetminTravel))
        (Variables|Default|SetminTravel (Math|Float|Absolute(Float) (Math|Vector|VectorLength (- (.TraceEnd (Collision|BreakHitResult _outhit_2)) (Variables|Default|GettargetLoc)))))
        (Variables|Default|SetnextMoveLoc (.TraceEnd (Collision|BreakHitResult _outhit_2)))))
    (CallFunction|TraceVertical)
    (bind _output_get (Variables|Default|SetcurTrace (+ (Variables|Default|GetcurTrace) 1)))
    (if (> _output_get 12)
      (Variables|Default|SetcurTrace 1)
      (Variables|Default|SetcurMoveLoc (Variables|Default|GetnextMoveLoc))
      (Variables|Default|SetminTravel 999999995904.0))
    (else
      (Variables|Default|SetcurMoveLoc (Variables|Default|GettargetLoc)))))

(event Custom|UpdateMovement
  (params (deltaTime :type Float%20%28double-precision%29))
  (bind _npcpawn (Variables|Default|GetNpcPawn))
  (if (Utilities|Operators|NotEqual(!=) :A (Variables|Default|GettargetLoc))
    (if (not (<= (Math|Float|Absolute(Float) (Math|Vector|VectorLength (- (Transformation|GetActorLocation (Variables|Default|GetNpcPawn)) (Variables|Default|GettargetLoc)))) 1.5e+02))
      (CallFunction|FindClosestPoint)
      (Transformation|SetActorRotation (Variables|Default|GetNpcPawn) (Math|Interpolation|RInterpTo (Transformation|GetActorRotation _npcpawn) (Math|Rotator|FindLookatRotation (Transformation|GetActorLocation _npcpawn) (Variables|Default|GetcurMoveLoc)) deltaTime 2e+01))
      (Default|WorldMoveandSlide (Variables|/Game/Blueprints/Actors/A-CharacterPawn.A-CharacterPawn_C|GetAC-ActorPawnMovement (Variables|Default|GetNpcPawn)) deltaTime (Math|Vector|GetUnitDirection(Vector) (Transformation|GetActorLocation (Variables|Default|GetNpcPawn)) (Variables|Default|GetcurMoveLoc)) 9e+02))))

(event EventBeginPlay
  (bind _asa_npc_character_pawn (Utilities|Casting|CastToA-NpcCharacterPawn (Components|GetOwner)))
  (Variables|Default|SetNpcPawn _asa_npc_character_pawn))

(event EventTick
  (params (DeltaSeconds :type Float%20%28single-precision%29))
  (CallFunction|UpdateMovement DeltaSeconds)
  (CallFunction|SetTargetLoc)
  (CallFunction|SetGravity)
  (CallFunction|AddGrav))