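; Movement component for a zero-gravity pawn, with forward and strafe thrust plus free rotation around the pawn's own up and camera right axes.
; Clamped input builds decaying thrust pulses that drive a swept world offset, nudged along a reflection-based direction on blocking hits.
; The local pawn relays its transform through server and cast events, and other copies interpolate toward it.
; ColForce computes a push-back velocity from PhysMesh hits, unused here.
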(event Custom|OnServerUpdatePos
  (params (Target :type Scene%20Component%20Object%20Reference) (NewLocation :type Vector) (NewRotation :type Rotator))
  (CallFunction|CastUpdatePos Target NewLocation NewRotation))

(event Custom|CastUpdatePos
  (params (Target :type Scene%20Component%20Object%20Reference) (NewLocation :type Vector) (NewRotation :type Rotator))
  (bind _pawncam (Variables|Default|GetPawnCam))
  (Variables|/Game/Blueprints/Pawns/P-PlayerCam.P-PlayerCam_C|SetglobalLocCast _pawncam NewLocation)
  (Variables|/Game/Blueprints/Pawns/P-PlayerCam.P-PlayerCam_C|SetglobalRotCast _pawncam NewRotation))

(event Custom|ColForce
  (bind _pawncam (Variables|Default|GetPawnCam))
  (bind _pawnactor (Variables|/Game/Blueprints/Pawns/P-PlayerCam.P-PlayerCam_C|GetPawnActor _pawncam))
  (bind _returnvalue (Transformation|GetActorLocation _pawnactor))
  ;[0.15 0.15 0.15 0.5] Change to an event that is called when the ship sweeps(ship will sweep, and all 'physObjects it collides with will have this event called on them(gonna have to make a weigh scale like HalfLife?))
  (bind _outhit (Collision|CapsuleTraceByChannel _returnvalue _returnvalue 2e+01 5e+01 "TraceTypeQuery1" false 0 "None"))
  (if (Utilities|Enum|Equal(Enum) (Utilities|GetObjectName (.HitComponent (Collision|BreakHitResult _outhit))) "PhysMesh")
    (Variables|Default|SetPushBackVel (* (Math|Vector|GetUnitDirection(Vector) (.ImpactPoint (Collision|BreakHitResult _outhit)) (.TraceStart (Collision|BreakHitResult _outhit))) 5e+01))))

(event Custom|MoveAndSlide
  (params (deltaTime :type Float%20%28double-precision%29) (Vel :type Vector))
  (bind _sweephitresult (Transformation|AddActorWorldOffset (Variables|/Game/Blueprints/Pawns/P-PlayerCam.P-PlayerCam_C|GetPawnActor (Variables|Default|GetPawnCam)) (* deltaTime Vel 9e+02) true))
  (if (.bBlockingHit (Collision|BreakHitResult _sweephitresult))
    (Transformation|AddActorWorldOffset (Variables|/Game/Blueprints/Pawns/P-PlayerCam.P-PlayerCam_C|GetPawnActor (Variables|Default|GetPawnCam)) (* (Math|Vector|GetUnitDirection(Vector) (Transformation|GetActorLocation (Variables|/Game/Blueprints/Pawns/P-PlayerCam.P-PlayerCam_C|GetPawnActor (Variables|Default|GetPawnCam))) (+ (.Location (Collision|BreakHitResult _sweephitresult)) (Math|Vector|GetReflectionVector (Math|Vector|GetUnitDirection(Vector) (.TraceStart (Collision|BreakHitResult _sweephitresult)) (.TraceEnd (Collision|BreakHitResult _sweephitresult))) (.Normal (Collision|BreakHitResult _sweephitresult))))) 1e+01) true)))

(event Custom|TickSidePowerCalc
  (params (deltaTime :type Float%20%28double-precision%29))
  (bind _returnvalue (* deltaTime 4.0))
  (bind _output_get (Variables|Default|SetSidePulse (Math|Float|Clamp(Float) (+ (* _returnvalue (* 2.0 (Variables|Default|GetSideInput))) (Variables|Default|GetSidePulse)) -1.0)))
  (if (> _output_get 0.0)
    (Variables|Default|SetSidePulse (Math|Float|Clamp(Float) (- _output_get _returnvalue)))
    (elif (< _output_get 0.0)
      (Variables|Default|SetSidePulse (Math|Float|Clamp(Float) (+ _output_get _returnvalue) -1.0 0.0)))))

(event Custom|TickFwdPowerCalc
  (params (deltaTime :type Float%20%28double-precision%29))
  (bind _returnvalue (* deltaTime 4.0))
  (bind _output_get (Variables|Default|SetFwdPulse (Math|Float|Clamp(Float) (+ (* _returnvalue (* 2.0 (Variables|Default|GetFwdInput))) (Variables|Default|GetFwdPulse)) -1.0)))
  (if (> _output_get 0.0)
    (Variables|Default|SetFwdPulse (Math|Float|Clamp(Float) (- _output_get _returnvalue)))
    (elif (< _output_get 0.0)
      (Variables|Default|SetFwdPulse (Math|Float|Clamp(Float) (+ _output_get _returnvalue) -1.0 0.0)))))

(event EventBeginPlay
  (|CallParentFunction))

(event EventTick
  (params (DeltaSeconds :type Float%20%28single-precision%29))
  (bind _pawncam (Variables|Default|GetPawnCam))
  (bind _pawncam_2 (Variables|Default|GetPawnCam))
  (bind _pawncam_3 (Variables|Default|GetPawnCam))
  (bind _pawnactor (Variables|/Game/Blueprints/Pawns/P-PlayerCam.P-PlayerCam_C|GetPawnActor _pawncam_2))
  (bind _rootcomponent (Variables|/Script/Engine.Actor|GetRootComponent _pawncam))
  (bind _pawnactor_2 (Variables|/Game/Blueprints/Pawns/P-PlayerCam.P-PlayerCam_C|GetPawnActor _pawncam_3))
  (bind _rootcomponent_2 (Variables|/Script/Engine.Actor|GetRootComponent _pawnactor_2))
  (bind _rootcomponent_3 (Variables|/Script/Engine.Actor|GetRootComponent _pawnactor))
  (if (Variables|/Game/Blueprints/Pawns/P-PlayerCam.P-PlayerCam_C|GetIsLocal (Variables|Default|GetPawnCam))
    (CallFunction|TickFwdPowerCalc DeltaSeconds)
    (CallFunction|TickSidePowerCalc DeltaSeconds)
    (CallFunction|MoveandSlide DeltaSeconds (+ (* (Math|Vector|GetForwardVector _rootcomponent) (Variables|Default|GetFwdPulse)) (* (Math|Vector|GetRightVector _rootcomponent) (Variables|Default|GetSidePulse))))
    (CallFunction|OnServerUpdatePos _rootcomponent_2 (Transformation|GetWorldLocation _rootcomponent_2) (Transformation|GetWorldRotation _rootcomponent_2))
    (else
      (Transformation|SetWorldLocation _rootcomponent_3 (Math|Interpolation|VInterpTo (Transformation|GetWorldLocation _rootcomponent_3) (Variables|/Game/Blueprints/Pawns/P-PlayerCam.P-PlayerCam_C|GetglobalLocCast _pawncam_2) 1.0 1.0) false false)
      (Transformation|SetWorldRotation _rootcomponent_3 (Math|Interpolation|RInterpTo (Transformation|GetWorldRotation _rootcomponent_3) (Variables|/Game/Blueprints/Pawns/P-PlayerCam.P-PlayerCam_C|GetglobalRotCast _pawncam_2) 1.0 1.0) false false))))

(event EventLocalLookUp
  (params (Ip :type Float%20%28double-precision%29))
  (bind _pawncam (Variables|Default|GetPawnCam))
  (bind _pawnactor (Variables|/Game/Blueprints/Pawns/P-PlayerCam.P-PlayerCam_C|GetPawnActor _pawncam))
  (Class|Actor|AddActorWorldRotation _pawnactor (Math|Vector|RotatorfromAxisandAngle (Math|Vector|GetRightVector (Transformation|GetWorldRotation (Variables|/Game/Blueprints/Pawns/A-PlayerPawn.A-PlayerPawn_C|GetCamPos _pawnactor))) (* Ip -1.0))))

(event EventLocalRotatePlayer
  (params (ValZ :type Float%20%28double-precision%29))
  (bind _pawncam (Variables|Default|GetPawnCam))
  (bind _pawnactor (Variables|/Game/Blueprints/Pawns/P-PlayerCam.P-PlayerCam_C|GetPawnActor _pawncam))
  (Class|Actor|AddActorWorldRotation _pawnactor (Math|Vector|RotatorfromAxisandAngle (Math|Vector|GetUpVector (Transformation|GetActorRotation _pawnactor)) ValZ)))

(event EventLocalAddMovementX
  (params (Ip :type Float%20%28double-precision%29))
  (Variables|Default|SetFwdInput (Math|Float|Clamp(Float) Ip -1.0)))

(event EventLocalAddMovementY
  (params (Ip :type Float%20%28double-precision%29))
  (Variables|Default|SetSideInput (Math|Float|Clamp(Float) Ip -1.0)))