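; Custom pawn movement component for on-foot play inside a ship's gravity area, handling walk, look, jump, slide and crouch.
; The local pawn ticks swept local-space offsets with reflection-based wall deflection, using traces for floor, gravity and uncrouch clearance.
; It detaches gravity outside the ship and flags driving availability in the drive area.
; Position, yaw and animation state pass through server-to-cast events, which remote copies apply directly without interpolation.
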(event Custom|OnServerUpdatePos
  (params (Pawn :type A-Player%20Pawn%20Object%20Reference) (Pos :type Vector) (Rot :type Rotator) (curXSpeed :type Float%20%28double-precision%29) (curYSpeed :type Float%20%28double-precision%29) (isInAir :type Boolean))
  (CallFunction|CastUpdatePos Pawn Pos Rot curXSpeed curYSpeed isInAir))

(event Custom|CastUpdatePos
  (params (Pawn :type A-Player%20Pawn%20Object%20Reference) (Pos :type Vector) (Rot :type Rotator) (curXSpeed :type Float%20%28double-precision%29) (curYSpeed :type Float%20%28double-precision%29) (isInAir :type Boolean))
  (bind _pawncam (Variables|Default|GetPawnCam))
  (Variables|/Game/Blueprints/Pawns/P-PlayerCam.P-PlayerCam_C|SetlocalLocCast _pawncam Pos)
  (Variables|/Game/Blueprints/Pawns/P-PlayerCam.P-PlayerCam_C|SetlocalRotCast _pawncam Rot)
  (Variables|/Game/Blueprints/Pawns/P-PlayerCam.P-PlayerCam_C|SetanimXSpeed _pawncam curXSpeed)
  (Variables|/Game/Blueprints/Pawns/P-PlayerCam.P-PlayerCam_C|SetanimYSpeed _pawncam curYSpeed)
  (Variables|/Game/Blueprints/Pawns/P-PlayerCam.P-PlayerCam_C|SetanimIsInAir _pawncam isInAir))

(event Custom|UpdateCol
  (bind _pawncam (Variables|Default|GetPawnCam))
  (bind _pawnactor (Variables|/Game/Blueprints/Pawns/P-PlayerCam.P-PlayerCam_C|GetPawnActor _pawncam))
  (bind _base (Variables|/Game/Blueprints/Pawns/A-PlayerPawn.A-PlayerPawn_C|GetBase _pawnactor))
  (if (or (Variables|Default|GetisSlide) (Variables|Default|GetisCrouch))
    (if (!= (Variables|/Script/Engine.CapsuleComponent|GetCapsuleHalfHeight _base) 25.0)
      (Components|Capsule|SetCapsuleHalfHeight _base 25.0 false)
      (Transformation|SetRelativeLocation (Variables|/Game/Blueprints/Pawns/A-PlayerPawn.A-PlayerPawn_C|GetOnFloorColEnd _pawnactor) "0.000000,0.000000,-14.000000" false false)
      (Transformation|SetRelativeLocation (Variables|/Game/Blueprints/Pawns/A-PlayerPawn.A-PlayerPawn_C|GetOnFloorCheck _pawnactor) "0.000000,0.000000,-17.000000" false false))))

(event Custom|Uncrouch
  (params (deltaTime :type Float%20%28single-precision%29)))

(event Custom|CheckIfGravArea
  (if (not (Utilities|Array|ContainsItem (Collision|GetOverlappingActors (Variables|/Game/Blueprints/Pawns/P-PlayerCam.P-PlayerCam_C|GetPawnActor (Variables|Default|GetPawnCam)) 0 :!class /Script/Engine.Actor) (Variables|/Game/Blueprints/Pawns/P-PlayerCam.P-PlayerCam_C|GetShip (Variables|Default|GetPawnCam))))
    (Default|DetachfromGravity (Variables|Default|GetPawnCam))
    (Variables|Default|SetslideIp 0.0)
    (Variables|Default|SetjumpDir "0, 0, 0")
    (Variables|Default|SetslideDir "0, 0, 0")
    (Variables|Default|SetisJump false)))

(event Custom|FloorCheck
  (params (deltaTime :type Float%20%28double-precision%29))
  (bind _pawncam (Variables|Default|GetPawnCam))
  (bind _pawnactor (Variables|/Game/Blueprints/Pawns/P-PlayerCam.P-PlayerCam_C|GetPawnActor _pawncam))
  (bind _onfloorcheck (Variables|/Game/Blueprints/Pawns/A-PlayerPawn.A-PlayerPawn_C|GetOnFloorCheck _pawnactor))
  (bind _returnvalue (Transformation|GetWorldLocation _onfloorcheck))
  (bind _returnvalue_2 (Collision|SphereTraceByChannel _returnvalue _returnvalue 12.0 "TraceTypeQuery1" false 0 "None"))
  (if _returnvalue_2
    (Variables|Default|SetonFloor true)
    (Variables|Default|SetnoFloor false)
    (Variables|/Game/Blueprints/Pawns/A-PlayerPawn.A-PlayerPawn_C|SetisInAir (Variables|/Game/Blueprints/Pawns/P-PlayerCam.P-PlayerCam_C|GetPawnActor (Variables|Default|GetPawnCam)) false)
    (Variables|Default|SetcanJump true)
    (Variables|Default|SetjumpDir "0, 0, 0")
    (if (not (Variables|Default|GetisJump))
      (Variables|Default|SetjumpIp 0.0))
    (else
      (Variables|Default|SetonFloor false)
      (if (Variables|Default|GetnoFloor)
        (bind _output_get (Variables|Default|SetnoFloorTimer (+ deltaTime (Variables|Default|GetnoFloorTimer))))
        (if (> _output_get 0.2)
          (Variables|/Game/Blueprints/Pawns/A-PlayerPawn.A-PlayerPawn_C|SetisInAir (Variables|/Game/Blueprints/Pawns/P-PlayerCam.P-PlayerCam_C|GetPawnActor (Variables|Default|GetPawnCam)) true))
        (else
          (Variables|Default|SetnoFloor true)
          (Variables|Default|SetnoFloorTimer 0.0))))))

(event Custom|AddGravity
  (if (not (Variables|Default|GetonFloor))
    (Variables|Default|SetgravityScale 1.0)
    (else
      (Variables|Default|SetgravityScale 0.0))))

(event Custom|CanDrive
  (bind _pawncam (Variables|Default|GetPawnCam))
  (bind _ship (Variables|/Game/Blueprints/Pawns/P-PlayerCam.P-PlayerCam_C|GetShip _pawncam))
  (if (Utilities|Array|ContainsItem (Class|Actor|GetOverlappingComponents (Variables|/Game/Blueprints/Pawns/P-PlayerCam.P-PlayerCam_C|GetPawnActor (Variables|Default|GetPawnCam))) (Variables|/Game/Blueprints/Pawns/A-BaseShip.A-BaseShip_C|GetDriveArea _ship))
    (if (not (Variables|/Game/Blueprints/Pawns/A-BaseShip.A-BaseShip_C|GethasDriver _ship))
      (Variables|/Game/Blueprints/Pawns/P-PlayerCam.P-PlayerCam_C|SetcanDrive (Variables|Default|GetPawnCam) true)
      (else
        (Variables|/Game/Blueprints/Pawns/P-PlayerCam.P-PlayerCam_C|SetcanDrive (Variables|Default|GetPawnCam) false :!label _label)))
    (else
      (goto _label))))

(event Custom|MoveAndSlide
  (params (DeltaTime :type Float%20%28single-precision%29))
  (bind _pawncam (Variables|Default|GetPawnCam))
  (bind _pawncam_2 (Variables|Default|GetPawnCam))
  (bind _pawnactor (Variables|/Game/Blueprints/Pawns/P-PlayerCam.P-PlayerCam_C|GetPawnActor _pawncam))
  (bind _pawnactor_2 (Variables|/Game/Blueprints/Pawns/P-PlayerCam.P-PlayerCam_C|GetPawnActor _pawncam_2))
  (CallFunction|MoveandSlideJumpDir DeltaTime)
  (CallFunction|MoveandSlideSlideDir DeltaTime)
  (Transformation|AddActorLocalOffset (Variables|/Game/Blueprints/Pawns/P-PlayerCam.P-PlayerCam_C|GetPawnActor (Variables|Default|GetPawnCam)) (* DeltaTime (Math|Vector|MakeVector 0.0 0.0 (+ (* (Variables|Default|GetjumpIp) 2.7e+03) (* -1.8e+03 (Variables|Default|GetgravityScale)) (* (Variables|Default|GetfloorFixIp) 2.7e+03)))) true false)
  (if (and (Variables|Default|GetonFloor) (not (Variables|Default|GetisSlide)))
    (bind _sweephitresult (Transformation|AddActorLocalOffset _pawnactor_2 (* DeltaTime (Math|Vector|MakeVector (* (Variables|Default|GetxIp) 6e+02) (* (Variables|Default|GetyIp) 6e+02) 0.0)) true false))
    (if (.bBlockingHit (Collision|BreakHitResult _sweephitresult))
      (Transformation|AddActorWorldOffset _pawnactor_2 (* (Math|Vector|GetUnitDirection(Vector) (Transformation|GetActorLocation (Variables|/Game/Blueprints/Pawns/P-PlayerCam.P-PlayerCam_C|GetPawnActor (Variables|Default|GetPawnCam))) (+ (.Location (Collision|BreakHitResult _sweephitresult)) (Math|Vector|GetReflectionVector (Math|Vector|GetUnitDirection(Vector) (.TraceStart (Collision|BreakHitResult _sweephitresult)) (.TraceEnd (Collision|BreakHitResult _sweephitresult))) (.Normal (Collision|BreakHitResult _sweephitresult))))) 6e+02 DeltaTime) true))
    (else
      (bind _sweephitresult_2 (Transformation|AddActorLocalOffset _pawnactor (* DeltaTime (Math|Vector|MakeVector (* (Variables|Default|GetxIp) 3.5e+02) (* (Variables|Default|GetyIp) 3.5e+02) 0.0)) true false))
      (if (.bBlockingHit (Collision|BreakHitResult _sweephitresult_2))
        (Transformation|AddActorWorldOffset _pawnactor (* (Math|Vector|GetUnitDirection(Vector) (Transformation|GetActorLocation (Variables|/Game/Blueprints/Pawns/P-PlayerCam.P-PlayerCam_C|GetPawnActor (Variables|Default|GetPawnCam))) (+ (.Location (Collision|BreakHitResult _sweephitresult_2)) (Math|Vector|GetReflectionVector (Math|Vector|GetUnitDirection(Vector) (.TraceStart (Collision|BreakHitResult _sweephitresult_2)) (.TraceEnd (Collision|BreakHitResult _sweephitresult_2))) (.Normal (Collision|BreakHitResult _sweephitresult_2))))) 6e+02 DeltaTime) true)))))

(event Custom|MoveAndSlideJumpDir
  (params (deltaTime :type Float%20%28double-precision%29))
  (bind _pawncam (Variables|Default|GetPawnCam))
  (bind _pawnactor (Variables|/Game/Blueprints/Pawns/P-PlayerCam.P-PlayerCam_C|GetPawnActor _pawncam))
  (bind _sweephitresult (Transformation|AddRelativeLocation (Variables|/Script/Engine.Actor|GetRootComponent (Variables|/Game/Blueprints/Pawns/P-PlayerCam.P-PlayerCam_C|GetPawnActor (Variables|Default|GetPawnCam))) (* (Variables|Default|GetjumpDir) (+ deltaTime (Variables|Default|GetjumpIp)) 1e+01) true false))
  (if (.bBlockingHit (Collision|BreakHitResult _sweephitresult))
    (Transformation|AddActorWorldOffset _pawnactor (* (Math|Vector|GetUnitDirection(Vector) (Transformation|GetActorLocation _pawnactor) (+ (.Location (Collision|BreakHitResult _sweephitresult)) (Math|Vector|GetReflectionVector (Math|Vector|GetUnitDirection(Vector) (.TraceStart (Collision|BreakHitResult _sweephitresult)) (.TraceEnd (Collision|BreakHitResult _sweephitresult))) (.Normal (Collision|BreakHitResult _sweephitresult))))) 6e+02 deltaTime) true))
  (Variables|Default|SetjumpIp (Math|Float|Clamp(Float) (- (Variables|Default|GetjumpIp) deltaTime))))

(event Custom|MoveAndSlideSlideDir
  (params (deltaTime :type Float%20%28double-precision%29))
  (bind _pawncam (Variables|Default|GetPawnCam))
  (bind _pawnactor (Variables|/Game/Blueprints/Pawns/P-PlayerCam.P-PlayerCam_C|GetPawnActor _pawncam))
  (bind _sweephitresult (Transformation|AddRelativeLocation (Variables|/Script/Engine.Actor|GetRootComponent (Variables|/Game/Blueprints/Pawns/P-PlayerCam.P-PlayerCam_C|GetPawnActor (Variables|Default|GetPawnCam))) (* (Variables|Default|GetslideDir) (+ deltaTime (Variables|Default|GetslideIp)) 1e+02) true false))
  (if (.bBlockingHit (Collision|BreakHitResult _sweephitresult))
    (Transformation|AddActorWorldOffset _pawnactor (* (Math|Vector|GetUnitDirection(Vector) (Transformation|GetActorLocation _pawnactor) (+ (.Location (Collision|BreakHitResult _sweephitresult)) (Math|Vector|GetReflectionVector (Math|Vector|GetUnitDirection(Vector) (.TraceStart (Collision|BreakHitResult _sweephitresult)) (.TraceEnd (Collision|BreakHitResult _sweephitresult))) (.Normal (Collision|BreakHitResult _sweephitresult))))) 6e+02 deltaTime) true))
  (Variables|Default|SetslideIp (Math|Float|Clamp(Float) (- (Variables|Default|GetslideIp) deltaTime)))
  (if (== (Variables|Default|GetslideIp) 0.0)
    (if (Variables|Default|GetisSlide)
      (CallFunction|LocalCrouch deltaTime))))

(event Custom|FloorCol
  (bind _pawncam (Variables|Default|GetPawnCam))
  (bind _pawnactor (Variables|/Game/Blueprints/Pawns/P-PlayerCam.P-PlayerCam_C|GetPawnActor _pawncam))
  (bind _returnvalue (Collision|SphereTraceByChannel (Transformation|GetWorldLocation (Variables|/Game/Blueprints/Pawns/A-PlayerPawn.A-PlayerPawn_C|GetOnFloorCol _pawnactor)) (Transformation|GetWorldLocation (Variables|/Game/Blueprints/Pawns/A-PlayerPawn.A-PlayerPawn_C|GetOnFloorColEnd _pawnactor)) 12.0 "TraceTypeQuery1" false 0 "None"))
  (if _returnvalue
    (Variables|Default|SetfloorFixIp 0.5)
    (else
      (Variables|Default|SetfloorFixIp 0.0))))

(event EventBeginPlay
  (|CallParentFunction))

(event EventTick
  (params (DeltaSeconds :type Float%20%28single-precision%29))
  (bind _pawncam (Variables|Default|GetPawnCam))
  (bind _pawncam_2 (Variables|Default|GetPawnCam))
  (bind _pawnactor (Variables|/Game/Blueprints/Pawns/P-PlayerCam.P-PlayerCam_C|GetPawnActor _pawncam))
  (bind _pawnactor_2 (Variables|/Game/Blueprints/Pawns/P-PlayerCam.P-PlayerCam_C|GetPawnActor _pawncam_2))
  (bind _rootcomponent (Variables|/Script/Engine.Actor|GetRootComponent _pawnactor_2))
  (bind _rootcomponent_2 (Variables|/Script/Engine.Actor|GetRootComponent _pawnactor))
  (if (Variables|/Game/Blueprints/Pawns/P-PlayerCam.P-PlayerCam_C|GetIsLocal (Variables|Default|GetPawnCam))
    (CallFunction|UpdateCol)
    (CallFunction|AddGravity)
    (CallFunction|CheckifGravArea)
    (CallFunction|CanDrive)
    (CallFunction|MoveandSlide DeltaSeconds)
    (CallFunction|OnServerUpdatePos _pawnactor_2 (Variables|/Script/Engine.SceneComponent|GetRelativeLocation _rootcomponent) (Math|Rotator|MakeRotator 0.0 0.0 (.yaw (Variables|/Script/Engine.SceneComponent|GetRelativeRotation _rootcomponent))) (Variables|/Game/Blueprints/Pawns/A-PlayerPawn.A-PlayerPawn_C|GetcurXSpeed _pawnactor_2) (Variables|/Game/Blueprints/Pawns/A-PlayerPawn.A-PlayerPawn_C|GetcurYSpeed _pawnactor_2) (Variables|/Game/Blueprints/Pawns/A-PlayerPawn.A-PlayerPawn_C|GetisInAir _pawnactor_2))
    (CallFunction|FloorCheck DeltaSeconds)
    (CallFunction|FloorCol)
    (else
      (Transformation|SetRelativeRotation _rootcomponent_2 (Variables|/Game/Blueprints/Pawns/P-PlayerCam.P-PlayerCam_C|GetlocalRotCast _pawncam) false false)
      (Transformation|SetRelativeLocation _rootcomponent_2 (Variables|/Game/Blueprints/Pawns/P-PlayerCam.P-PlayerCam_C|GetlocalLocCast _pawncam) false false)
      (Variables|/Game/Blueprints/Pawns/A-PlayerPawn.A-PlayerPawn_C|SetcurXSpeed _pawnactor (Variables|/Game/Blueprints/Pawns/P-PlayerCam.P-PlayerCam_C|GetanimXSpeed _pawncam))
      (Variables|/Game/Blueprints/Pawns/A-PlayerPawn.A-PlayerPawn_C|SetcurYSpeed _pawnactor (Variables|/Game/Blueprints/Pawns/P-PlayerCam.P-PlayerCam_C|GetanimYSpeed _pawncam))
      (Variables|/Game/Blueprints/Pawns/A-PlayerPawn.A-PlayerPawn_C|SetisInAir _pawnactor (Variables|/Game/Blueprints/Pawns/P-PlayerCam.P-PlayerCam_C|GetanimIsInAir _pawncam)))))

(event EventLocalRotatePlayer
  (params (ValZ :type Float%20%28double-precision%29))
  (bind _pawncam (Variables|Default|GetPawnCam))
  (bind _pawnactor (Variables|/Game/Blueprints/Pawns/P-PlayerCam.P-PlayerCam_C|GetPawnActor _pawncam))
  (bind _rootcomponent (Variables|/Script/Engine.Actor|GetRootComponent _pawnactor))
  (Transformation|SetRelativeRotation _rootcomponent (Math|Rotator|MakeRotator 0.0 0.0 (+ ValZ (.yaw (Variables|/Script/Engine.SceneComponent|GetRelativeRotation _rootcomponent)))) false false))

(event EventLocalLookUp
  (params (Ip :type Float%20%28double-precision%29))
  (bind _pawncam (Variables|Default|GetPawnCam))
  (bind _pawnactor (Variables|/Game/Blueprints/Pawns/P-PlayerCam.P-PlayerCam_C|GetPawnActor _pawncam))
  (bind _cameraroot (Variables|/Game/Blueprints/Pawns/A-PlayerPawn.A-PlayerPawn_C|GetCameraRoot _pawnactor))
  (Transformation|SetRelativeRotation _cameraroot (Math|Rotator|MakeRotator 0.0 (Math|Float|Clamp(Float) (+ Ip (.pitch (Variables|/Script/Engine.SceneComponent|GetRelativeRotation _cameraroot))) -9e+01 9e+01) 0.0) false false))

(event EventLocalJump
  (params (Ip :type Boolean))
  (bind _pawncam (Variables|Default|GetPawnCam))
  (bind _xip (Variables|Default|GetxIp))
  (bind _yip (Variables|Default|GetyIp))
  (bind _pawnactor (Variables|/Game/Blueprints/Pawns/P-PlayerCam.P-PlayerCam_C|GetPawnActor _pawncam))
  (bind _rootcomponent (Variables|/Script/Engine.Actor|GetRootComponent _pawnactor))
  (bind _relativerotation (Variables|/Script/Engine.SceneComponent|GetRelativeRotation _rootcomponent))
  (bind _returnvalue (Math|Vector|GetForwardVector _relativerotation))
  (bind _returnvalue_2 (Math|Vector|GetRightVector _relativerotation))
  (bind _returnvalue_3 (* _returnvalue _xip))
  (bind _returnvalue_4 (* _returnvalue_2 _yip))
  (bind _returnvalue_5 (+ _returnvalue_3 _returnvalue_4))
  (if (Variables|Default|GetcanJump)
    (Variables|Default|SetcanJump false)
    (Variables|Default|SetjumpIp 1.0)
    (Variables|/Game/Blueprints/Pawns/A-PlayerPawn.A-PlayerPawn_C|SetisInAir _pawnactor true)
    (if (Variables|Default|GetisSlide)
      (Variables|Default|SetjumpDir (* _returnvalue_5 2.0))
      (else
        (Variables|Default|SetjumpDir _returnvalue_5)))
    (Variables|Default|SetisJump true)
    (Utilities|FlowControl|Delay 0.1)
    (Variables|Default|SetisJump false)))

(event EventLocalSlide
  (bind _pawncam (Variables|Default|GetPawnCam))
  (bind _pawnactor (Variables|/Game/Blueprints/Pawns/P-PlayerCam.P-PlayerCam_C|GetPawnActor _pawncam))
  (bind _rootcomponent (Variables|/Script/Engine.Actor|GetRootComponent _pawnactor))
  (bind _relativerotation (Variables|/Script/Engine.SceneComponent|GetRelativeRotation _rootcomponent))
  (if (and (not (Variables|Default|GetisSlide)) (or (!= (Variables|Default|GetxIp) 0.0) (!= (Variables|Default|GetyIp) 0.0)))
    (Variables|Default|SetisSlide true)
    (Variables|Default|SetslideIp 0.4)
    (Variables|Default|SetslideDir (+ (* (Math|Vector|GetForwardVector _relativerotation) (Variables|Default|GetxIp)) (* (Math|Vector|GetRightVector _relativerotation) (Variables|Default|GetyIp))))
    (Variables|Default|SetisCrouch true)
    (else
      (Variables|Default|SetisSlide false)
      (Variables|Default|SetslideIp 0.0)
      (Variables|Default|SetslideDir "0, 0, 0")
      (Variables|Default|SetisCrouch false))))

(event EventLocalCrouch
  (params (time :type Float%20%28double-precision%29))
  (bind _pawncam (Variables|Default|GetPawnCam))
  (bind _pawnactor (Variables|/Game/Blueprints/Pawns/P-PlayerCam.P-PlayerCam_C|GetPawnActor _pawncam))
  (bind _base (Variables|/Game/Blueprints/Pawns/A-PlayerPawn.A-PlayerPawn_C|GetBase _pawnactor))
  (if (Variables|Default|GetisSlide)
    (Variables|Default|SetisSlide false)
    (Variables|Default|SetslideIp 0.0)
    (Variables|Default|SetslideDir "0, 0, 0")
    (bind _can (CallFunction|CanUncrouch :!label _label))
    (if (and _can (!= (Variables|/Script/Engine.CapsuleComponent|GetCapsuleHalfHeight _base) 4e+01))
      (Transformation|AddActorLocalOffset (Variables|/Game/Blueprints/Pawns/P-PlayerCam.P-PlayerCam_C|GetPawnActor (Variables|Default|GetPawnCam)) (* time (Math|Vector|MakeVector 0.0 0.0 2.7e+03)) true false)
      (Components|Capsule|SetCapsuleHalfHeight _base 4e+01 false)
      (Transformation|SetRelativeLocation (Variables|/Game/Blueprints/Pawns/A-PlayerPawn.A-PlayerPawn_C|GetOnFloorColEnd _pawnactor) "0.000000,0.000000,-29.000000" false false)
      (Transformation|SetRelativeLocation (Variables|/Game/Blueprints/Pawns/A-PlayerPawn.A-PlayerPawn_C|GetOnFloorCheck _pawnactor) "0.000000,0.000000,-32.000000" false false)
      (Variables|Default|SetisCrouch false))
    (elif (Variables|Default|GetisCrouch)
      (goto _label)
      (else
        (Variables|Default|SetisCrouch true)))))

(event EventLocalAddMovementX
  (params (Ip :type Float%20%28double-precision%29))
  (bind _output_get (Variables|Default|SetxIp Ip))
  (Variables|/Game/Blueprints/Pawns/A-PlayerPawn.A-PlayerPawn_C|SetcurXSpeed (Variables|/Game/Blueprints/Pawns/P-PlayerCam.P-PlayerCam_C|GetPawnActor (Variables|Default|GetPawnCam)) _output_get))

(event EventLocalAddMovementY
  (params (Ip :type Float%20%28double-precision%29))
  (bind _output_get (Variables|Default|SetyIp Ip))
  (Variables|/Game/Blueprints/Pawns/A-PlayerPawn.A-PlayerPawn_C|SetcurYSpeed (Variables|/Game/Blueprints/Pawns/P-PlayerCam.P-PlayerCam_C|GetPawnActor (Variables|Default|GetPawnCam)) _output_get))

(fn CanUncrouch
  (bind _pawncam (Variables|Default|GetPawnCam))
  (bind _pawnactor (Variables|/Game/Blueprints/Pawns/P-PlayerCam.P-PlayerCam_C|GetPawnActor _pawncam))
  (bind _returnvalue (Collision|LineTraceByChannel (Transformation|GetWorldLocation (Variables|/Game/Blueprints/Pawns/A-PlayerPawn.A-PlayerPawn_C|GetRoofCheck _pawnactor)) (Transformation|GetWorldLocation (Variables|/Game/Blueprints/Pawns/A-PlayerPawn.A-PlayerPawn_C|GetRoofCheckEnd _pawnactor)) "TraceTypeQuery1" false 0 "None"))
  (if _returnvalue
    (return false)
    (else
      (return true))))