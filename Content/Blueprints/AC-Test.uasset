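; Test actor component that prints placeholder debug strings, apparently to exercise Delay behaviour.
; Tick calls four custom events every frame, each with its own Delay before a print, so pending delays throttle three messages to about once a second and one to a faster rate.
; BeginPlay is empty, and disconnected leftover timer logic that would print and destroy the component never runs.
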(event Custom|Ev1
  (Utilities|FlowControl|Delay 1.0)
  (Development|PrintString "Hello"))

(event Custom|Ev4
  (Utilities|FlowControl|Delay 0.1)
  (Development|PrintString "!!!!!!!!!!"))

(event Custom|Ev2
  (Utilities|FlowControl|Delay 1.0)
  (Development|PrintString "There"))

(event Custom|Ev3
  (Utilities|FlowControl|Delay 1.0)
  (Development|PrintString "------"))

(event EventBeginPlay)

(event EventTick
  (params (DeltaSeconds :type Float%20%28single-precision%29))
  (CallFunction|Ev1)
  (CallFunction|Ev2)
  (CallFunction|Ev3)
  (CallFunction|Ev4))