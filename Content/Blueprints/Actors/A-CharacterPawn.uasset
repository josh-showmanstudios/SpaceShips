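; A-CharacterPawn is a character pawn that holds movement and animation state and exposes its collision probe components to other systems.
; On BeginPlay it starts airborne and not driving, then registers itself with the ABP-CharPawnMale animation blueprint.
; Setter events update speed, air, drive, capsule height and crouch probe offsets.
; Getters hand out the movement component, camera points, weight class and floor, roof and body check components.
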(event EventBeginPlay
  (Variables|Default|SetisInAir true)
  (Variables|Default|SetisDrive false)
  (bind _asabp_char_pawn_male (Utilities|Casting|CastToABP-CharPawnMale (Components|SkeletalMesh|GetAnimInstance (Variables|Default|GetSkeletalMesh))))
  (Default|SetChar _asabp_char_pawn_male self))

(event EventSetBaseCapsuleHeight
  (params (CapsuleHalfHeight :type Float%20%28double-precision%29))
  (Components|Capsule|SetCapsuleHalfHeight (Variables|Default|GetBase) CapsuleHalfHeight false))

(event EventSetCurrentSpeedY
  (params (CurYSpeed :type Float%20%28double-precision%29))
  (Variables|Default|SetcurSpeedY CurYSpeed))

(event EventSetCurrentSpeedX
  (params (CurXSpeed :type Float%20%28double-precision%29))
  (Variables|Default|SetcurSpeedX CurXSpeed))

(event EventSetIsinAir
  (params (IsInAir :type Boolean))
  (Variables|Default|SetisInAir IsInAir))

(event EventSetAnimationVariables
  (params (CurXSpeed :type Float%20%28double-precision%29) (CurYSpeed :type Float%20%28double-precision%29) (IsInAir :type Boolean))
  (Variables|Default|SetcurSpeedX CurXSpeed)
  (Variables|Default|SetcurSpeedY CurYSpeed)
  (Variables|Default|SetisInAir IsInAir))

(event EventSetIsDrive
  (params (IsDrive :type Boolean))
  (Variables|Default|SetisDrive IsDrive))

(event EventSetCrouchCollision
  (params (BodyColEndZ :type Float%20%28double-precision%29) (OnFLoorCheckZ :type Float%20%28double-precision%29))
  (Transformation|SetRelativeLocation (Variables|Default|GetBodyColEnd) (Math|Vector|MakeVector 0.0 0.0 BodyColEndZ) false false)
  (Transformation|SetRelativeLocation (Variables|Default|GetOnFloorCheck) (Math|Vector|MakeVector 0.0 0.0 OnFLoorCheckZ) false false)
  (Transformation|SetRelativeLocation (Variables|Default|GetGravityOnFloorCheck) (Math|Vector|MakeVector 0.0 0.0 (- OnFLoorCheckZ 18.0)) false false))

(fn ConstructionScript)

(fn GetActorMovement
  (return (Variables|Default|GetAC-ActorPawnMovement)))

(fn GetAnimationVariables
  (return (Variables|Default|GetcurSpeedX) (Variables|Default|GetcurSpeedY) (Variables|Default|GetisInAir)))

(fn GetBaseCapsuleHeight
  (return (Variables|/Script/Engine.CapsuleComponent|GetCapsuleHalfHeight (Variables|Default|GetBase))))

(fn GetBodyCollisionComponents
  (return (Variables|Default|GetBodyColTop) (Variables|Default|GetBodyColEnd)))

(fn GetCameraPosition
  (return (Variables|Default|GetCamPos)))

(fn GetCameraRoot
  (return (Variables|Default|GetCameraRoot)))

(fn GetFloorCheckComponentsV1
  (return 0 0))

(fn GetFloorCheckComponentsV2
  (return (Variables|Default|GetBodyColEnd) (Variables|Default|GetOnFloorCheck)))

(fn GetGravityFloorCheck
  (return (Variables|Default|GetOnFloorCheck) (Variables|Default|GetGravityOnFloorCheck)))

(fn GetHeadtoToe
  (return (Variables|Default|GetRoofCheck) (Variables|Default|GetBodyColEnd)))

(fn GetIsDrive
  (return (Variables|Default|GetisDrive)))

(fn GetIsinAIr
  (return (Variables|Default|GetisInAir)))

(fn GetNoGravCollisionBounds
  (return (Variables|Default|GetRoofCheckEnd) (Variables|Default|GetBodyColEnd)))

(fn GetRoofCheckComponents
  (return (Variables|Default|GetRoofCheck) (Variables|Default|GetRoofCheckEnd)))

(fn GetWeightClass
  (return (Variables|Default|GetWeightClass)))