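; A-NpcBasePawn is a base NPC pawn that exposes navigation control through its ACBoidNavAgent.
; Three wrapper events forward calls to the agent to set a target location, set a target actor, and update movement with a delta time.
; BeginPlay and the construction script only call their parents, and Tick is disabled, so the graph never drives movement itself.
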(event EventBeginPlay
  (|CallParentFunction))

(event EventCallSetTargetLoc
  (Default|SetTargetLoc (Variables|Default|GetAC-BoidNavAgent)))

(event EventTick
  (params (DeltaSeconds :type Float%20%28single-precision%29)))

(event EventCallUpdateMovement
  (params (deltaTime :type Float%20%28double-precision%29))
  (Default|UpdateMovement (Variables|Default|GetAC-BoidNavAgent) deltaTime))

(event EventCallSetTargetActor
  (params (TargetActor :type Actor%20Object%20Reference))
  (Default|SetTargetActor (Variables|Default|GetAC-BoidNavAgent) TargetActor))

(fn ConstructionScript
  (|CallParentFunction))