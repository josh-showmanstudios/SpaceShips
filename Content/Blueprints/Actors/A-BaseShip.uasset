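; Base ship actor that flies by thrust, pitch, yaw and roll inputs fed through clamped call events.
; Each Tick integrates velocity with drag and turns decaying input pulses into a combined rotation about the ship's axes, then applies both.
; The server passes location, rotation and velocity to CastLocRot, while clients also simulate and interpolate toward those values.
; Demo flight and tile-scan logic are disconnected, leaving Demo and MakeTiles inert.
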(event Custom|DemoPull
  (bind _root (Variables|Default|GetRoot))
  (bind _relativerotation (Variables|/Script/Engine.SceneComponent|GetRelativeRotation _root))
  (Transformation|SetRelativeRotation _root (Math|Interpolation|RInterpTo _relativerotation (Math|Rotator|CombineRotators _relativerotation (Math|Vector|RotatorfromAxisandAngle (Math|Vector|GetRightVector _relativerotation) 1.0)) 1.0 0.0) true false))

(event Custom|Demo
  (params (deltaTime :type Float%20%28double-precision%29))
  (if (Variables|Default|GetrunDemo)
    _))

(event Custom|DemoFwd
  (params (deltaTime :type Float%20%28double-precision%29))
  (Variables|Default|SetThrustInput 2.0)
  (CallFunction|PulsetoAdd deltaTime (* (Math|Vector|GetForwardVector (Variables|Default|GetRoot)) 5e+03)))

(event Custom|ThrustCall
  (params (Ip :type Float%20%28double-precision%29))
  (Variables|Default|SetThrustInput (Math|Float|Clamp(Float) Ip)))

(event Custom|RollCalc
  (params (deltaTime :type Float%20%28double-precision%29))
  (bind _output_get (Variables|Default|SetRollPulse (+ (Variables|Default|GetRollPulse) (* (* deltaTime 1.5) (Variables|Default|GetRollInput)))))
  (if (> _output_get 0.0)
    (Variables|Default|SetRollPulse (Math|Float|Clamp(Float) (- _output_get deltaTime)))
    (Variables|Default|SetRollPower (* (Variables|Default|GetRollPulse) 0.5) :!label _label)
    (elif (< _output_get 0.0)
      (Variables|Default|SetRollPulse (Math|Float|Clamp(Float) (+ _output_get deltaTime) -1.0 0.0))
      (goto _label)
      (else
        (Variables|Default|SetRollPower 0.0)))))

(event Custom|TurnCall
  (params (Ip :type Float%20%28single-precision%29))
  (Variables|Default|SetTurnInput (Math|Float|Clamp(Float) Ip -1.0)))

(event Custom|RollCall
  (params (Ip :type Float%20%28single-precision%29))
  (Variables|Default|SetRollInput (Math|Float|Clamp(Float) Ip -1.0)))

(event Custom|PullCall
  (params (Ip :type Float%20%28single-precision%29))
  (Variables|Default|SetPullInput (Math|Float|Clamp(Float) Ip -1.0)))

(event Custom|PullCalc
  (params (deltaTime :type Float%20%28double-precision%29))
  (bind _output_get (Variables|Default|SetPullPulse (+ (Variables|Default|GetPullPulse) (* (* deltaTime 1.5) (Variables|Default|GetPullInput)))))
  (if (> _output_get 0.0)
    (Variables|Default|SetPullPulse (Math|Float|Clamp(Float) (- _output_get deltaTime)))
    (Variables|Default|SetPullPower (* (Variables|Default|GetPullPulse) 0.5) :!label _label)
    (elif (< _output_get 0.0)
      (Variables|Default|SetPullPulse (Math|Float|Clamp(Float) (+ _output_get deltaTime) -1.0 0.0))
      (goto _label)
      (else
        (Variables|Default|SetPullPower 0.0)))))

(event Custom|AddThrustPulse
  (params (deltaTime :type Float%20%28double-precision%29))
  (CallFunction|PulsetoAdd deltaTime (Variables|Default|Getvelocity)))

(event Custom|CalcVelocity
  (params (deltaTime :type Float%20%28double-precision%29))
  (Variables|Default|Setvelocity (Math|Vector|ClampVectorSize (- (+ (* deltaTime (Variables|Default|GetThrustInput) (Math|Vector|GetForwardVector (Variables|Default|GetRoot)) 1e+03) (Variables|Default|Getvelocity)) (* (Math|Vector|Normalize (Variables|Default|Getvelocity) 0.001) deltaTime 5e+02)) -5e+03 5e+03)))

(event Custom|TurnCalc
  (params (deltaTime :type Float%20%28double-precision%29))
  (bind _output_get (Variables|Default|SetTurnPulse (+ (Variables|Default|GetTurnPulse) (* (* deltaTime 1.5) (Variables|Default|GetTurnInput)))))
  (if (> _output_get 0.0)
    (Variables|Default|SetTurnPulse (Math|Float|Clamp(Float) (- _output_get deltaTime)))
    (Variables|Default|SetTurnPower (* (Variables|Default|GetTurnPulse) 0.5) :!label _label)
    (elif (< _output_get 0.0)
      (Variables|Default|SetTurnPulse (Math|Float|Clamp(Float) (+ _output_get deltaTime) -1.0 0.0))
      (goto _label)
      (else
        (Variables|Default|SetTurnPower 0.0)))))

(event Custom|PulseToAdd
  (params (deltaTime :type Float%20%28double-precision%29) (InputDir :type Vector))
  (Transformation|AddActorWorldOffset (* deltaTime InputDir)))

(event Custom|SetHasDriver
  (params (hasDriver :type Boolean))
  (Variables|Default|SethasDriver hasDriver))

(event Custom|DemoTurn
  (bind _root (Variables|Default|GetRoot))
  (bind _relativerotation (Variables|/Script/Engine.SceneComponent|GetRelativeRotation _root))
  (Transformation|SetRelativeRotation _root (Math|Interpolation|RInterpTo _relativerotation (Math|Rotator|CombineRotators _relativerotation (Math|Vector|RotatorfromAxisandAngle (Math|Vector|GetUpVector _relativerotation) 1.0)) 1.0 0.0) true false))

(event Custom|DemoRoll
  (bind _root (Variables|Default|GetRoot))
  (bind _relativerotation (Variables|/Script/Engine.SceneComponent|GetRelativeRotation _root))
  (Transformation|SetRelativeRotation _root (Math|Interpolation|RInterpTo _relativerotation (Math|Rotator|CombineRotators _relativerotation (Math|Vector|RotatorfromAxisandAngle (Math|Vector|GetForwardVector _relativerotation) 1.0)) 1.0 0.0) true false))

(event Custom|CastLocRot
  (params (castLoc :type Vector) (castRot :type Rotator) (velocity :type Vector))
  (Variables|Default|SetcastLoc castLoc)
  (Variables|Default|SetcastRot castRot)
  (Variables|Default|SetcastVel velocity))

(event Custom|AddTurnVel
  (params (deltaTime :type Float%20%28double-precision%29))
  (bind _root (Variables|Default|GetRoot))
  (bind _relativerotation (Variables|/Script/Engine.SceneComponent|GetRelativeRotation _root))
  (Transformation|SetRelativeRotation _root (Math|Interpolation|RInterpTo _relativerotation (Math|Rotator|CombineRotators _relativerotation (Variables|Default|GetTurnVelocity)) deltaTime 1e+02) true false))

(event Custom|CalcTurnVel
  (bind _root (Variables|Default|GetRoot))
  (bind _relativerotation (Variables|/Script/Engine.SceneComponent|GetRelativeRotation _root))
  (Variables|Default|SetTurnVelocity (Math|Rotator|CombineRotators (Math|Rotator|CombineRotators (Math|Vector|RotatorfromAxisandAngle (Math|Vector|GetRightVector _relativerotation) (Variables|Default|GetPullPower)) (Math|Vector|RotatorfromAxisandAngle (Math|Vector|GetUpVector _relativerotation) (Variables|Default|GetTurnPower))) (Math|Vector|RotatorfromAxisandAngle (Math|Vector|GetForwardVector _relativerotation) (Variables|Default|GetRollPower)))))

(event EventBeginPlay
  (Variables|Default|SetdemoTimer 0.0)
  (if (Networking|IsServer)
    (Variables|Default|SetisServer true)
    (else
      (Variables|Default|SetisServer false))))

(event EventTick
  (params (DeltaSeconds :type Float%20%28single-precision%29))
  (CallFunction|CalcVelocity DeltaSeconds)
  (CallFunction|PullCalc DeltaSeconds)
  (CallFunction|RollCalc DeltaSeconds)
  (CallFunction|TurnCalc DeltaSeconds)
  (CallFunction|CalcTurnVel)
  (CallFunction|AddThrustPulse DeltaSeconds)
  (CallFunction|AddTurnVel DeltaSeconds)
  (if (Variables|Default|GetisServer)
    (CallFunction|CastLocRot (Transformation|GetWorldLocation (Variables|Transformation|GetRootComponent)) (Variables|/Script/Engine.SceneComponent|GetRelativeRotation (Variables|Default|GetRoot)) (Variables|Default|Getvelocity))
    (CallFunction|Demo DeltaSeconds)
    (else
      (Transformation|SetWorldLocation (Variables|Transformation|GetRootComponent) (Math|Interpolation|VInterpTo (Transformation|GetWorldLocation (Variables|Transformation|GetRootComponent)) (Variables|Default|GetcastLoc) 1.0 1.0) false false)
      (Transformation|SetRelativeRotation (Variables|Default|GetRoot) (Math|Interpolation|RInterpTo (Variables|/Script/Engine.SceneComponent|GetRelativeRotation (Variables|Default|GetRoot)) (Variables|Default|GetcastRot) 1.0 1.0) false false)
      (Variables|Default|Setvelocity (Variables|Default|GetcastVel)))))

(fn ConstructionScript)

(fn MakeTiles)