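; Player camera pawn that spawns a character, attaches to its camera position and routes Enhanced Input to it or a ship.
; Movement swaps between no-gravity, plane and sphere components as a sphere trace finds ship or planet gravity areas and attaches the character.
; Using while allowed to drive swaps pawn and ship mapping contexts.
; Server/Cast event pairs relay spawn and attachment changes, while cached transforms and animation values are exposed through getters.
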(event Custom|OnServerAttachSphere
  (params (Parent :type Scene%20Component%20Object%20Reference))
  ;[0.149 0.149 0.149 0.502] Attach and detach devents
  (CallFunction|CastAttachSphere Parent))

(event Custom|UpdateGlobalLocRot
  (params (NewLocation :type Vector) (NewRotation :type Rotator))
  (Variables|Cast|SetglobalLocCast NewLocation)
  (Variables|Cast|SetglobalRotCast NewRotation))

(event Custom|CheckHasChar
  (Utilities|IsValid (Variables|Default|GetOGControlledActor)
    (:Is%20Valid
      (bind _campos (Class|BPI-ActorPawn|GetCameraPosition(Message) (Variables|Default|GetOGControlledActor)))
      (Transformation|AttachComponentToComponent _campos "None" "KeepWorld" "KeepWorld" "KeepWorld" false)
      (Transformation|SetActorTransform (Math|Transform|MakeTransform (.location (Transformation|GetWorldTransform _campos)) (.rotation (Transformation|GetWorldTransform _campos)) "1.000000,1.000000,1.000000"))
      (Variables|Default|SetPawnMovementControl (Variables|Default|GetAC-NoGravControl))
      (Components|Tick|SetComponentTickEnabled (Variables|Default|GetAC-PlaneGravControl) false)
      (Components|Tick|SetComponentTickEnabled (Variables|Default|GetAC-NoGravControl) true)
      (Input|AddMappingContext (PlayerController|LocalPlayerSubsystems|GetEnhancedInputLocalPlayerSubsystem (Game|GetPlayerController 0)) "/Game/Input/IMC-Pawn.IMC-Pawn" 0 "(bIgnoreAllPressedKeysUntilRelease=True,bForceImmediately=False,bNotifyUserSettings=False)"))
    (:Is%20Not%20Valid
      (Utilities|FlowControl|Delay 0.1)
      (CallFunction|CheckHasChar))))

(event Custom|SpawnPawn
  (CallFunction|ServerSpawnPawn (Transformation|GetActorLocation) (Transformation|GetActorRotation))
  (Utilities|FlowControl|Delay 0.2)
  (CallFunction|CheckHasChar))

(event Custom|ServerShipThrust
  (params (Target :type A-Base%20Ship%20Object%20Reference) (ip :type Float%20%28double-precision%29))
  ;[0.15 0.15 0.15 0.5] Ship driving input
  (Default|ThrustCall Target ip))

(event Custom|CastShipThust
  (params (Target :type A-Base%20Ship%20Object%20Reference) (ip :type Float%20%28double-precision%29))
  ;[0.15 0.15 0.15 0.5] Ship driving input
  (Default|ThrustCall Target ip))

(event Custom|CastShipRoll
  (params (Target :type A-Base%20Ship%20Object%20Reference) (ip :type Float%20%28double-precision%29))
  ;[0.15 0.15 0.15 0.5] Ship driving input
  (Default|RollCall (stale Custom|ServerShipRoll Target) (stale Custom|ServerShipRoll ip)))

(event Custom|CastShipPull
  (params (Target :type A-Base%20Ship%20Object%20Reference) (ip :type Float%20%28double-precision%29))
  ;[0.15 0.15 0.15 0.5] Ship driving input
  (Default|PullCall (stale Custom|ServerShipPull Target) (stale Custom|ServerShipPull ip)))

(event Custom|CastShipTurn
  (params (Target :type A-Base%20Ship%20Object%20Reference) (ip :type Float%20%28double-precision%29))
  ;[0.15 0.15 0.15 0.5] Ship driving input
  (Default|TurnCall (stale Custom|ServerShipTurn Target) (stale Custom|ServerShipTurn ip)))

(event Custom|ServerShipRoll
  (params (Target :type A-Base%20Ship%20Object%20Reference) (ip :type Float%20%28double-precision%29))
  ;[0.15 0.15 0.15 0.5] Ship driving input
  (Default|RollCall Target ip))

(event Custom|CastDetach
  ;[0.149 0.149 0.149 0.502] Attach and detach devents
  (if (not (Variables|Default|GetIsLocal))
    (Transformation|DetachFromActor (Variables|Default|GetOGControlledActor) "KeepWorld" "KeepWorld" "KeepWorld")
    (Components|Tick|SetComponentTickEnabled (Variables|Default|GetAC-PlaneGravControl) false)
    (Components|Tick|SetComponentTickEnabled (Variables|Default|GetAC-NoGravControl) true)
    (Class|BPI-ActorPawn|SetAnimationVariables(Message) (Variables|Default|GetOGControlledActor) 0.0 0.0 true)))

(event Custom|ServerShipPull
  (params (Target :type A-Base%20Ship%20Object%20Reference) (ip :type Float%20%28double-precision%29))
  ;[0.15 0.15 0.15 0.5] Ship driving input
  (Default|PullCall Target ip))

(event Custom|PawnUse
  (bind _returnvalue (Game|GetPlayerController 0))
  (bind _returnvalue_2 (Game|GetPlayerController 0))
  (bind _returnvalue_3 (PlayerController|LocalPlayerSubsystems|GetEnhancedInputLocalPlayerSubsystem _returnvalue))
  (bind _returnvalue_4 (PlayerController|LocalPlayerSubsystems|GetEnhancedInputLocalPlayerSubsystem _returnvalue_2))
  ;[0.149 0.149 0.149 0.502] Comment
  (if (Variables|Default|GetisGrav)
    (bind _isdrive (Class|BPI-ActorPawn|GetIsDrive(Message) (Variables|Default|GetOGControlledActor)))
    (if _isdrive
      (Class|BPI-ActorPawn|SetIsDrive(Message) (Variables|Default|GetOGControlledActor) false)
      (Input|AddMappingContext _returnvalue_3 "/Game/Input/IMC-Pawn.IMC-Pawn" 0 "(bIgnoreAllPressedKeysUntilRelease=True,bForceImmediately=False,bNotifyUserSettings=False)")
      (Input|RemoveMappingContext _returnvalue_3 "/Game/Input/IMC-Ship.IMC-Ship" "(bIgnoreAllPressedKeysUntilRelease=True,bForceImmediately=False,bNotifyUserSettings=False)")
      (CallFunction|OnServerShipHasDriver (Variables|Default|GetshipActorREF) false)
      (elif (Variables|Default|GetcanDrive)
        (Class|BPI-ActorPawn|SetIsDrive(Message) (Variables|Default|GetOGControlledActor) true)
        (Input|AddMappingContext _returnvalue_4 "/Game/Input/IMC-Ship.IMC-Ship" 0 "(bIgnoreAllPressedKeysUntilRelease=True,bForceImmediately=False,bNotifyUserSettings=False)")
        (Input|RemoveMappingContext _returnvalue_4 "/Game/Input/IMC-Pawn.IMC-Pawn" "(bIgnoreAllPressedKeysUntilRelease=True,bForceImmediately=False,bNotifyUserSettings=False)")
        (CallFunction|OnServerShipHasDriver (Variables|Default|GetshipActorREF) true)))))

(event Custom|ServerShipTurn
  (params (Target :type A-Base%20Ship%20Object%20Reference) (ip :type Float%20%28double-precision%29))
  ;[0.15 0.15 0.15 0.5] Ship driving input
  (Default|TurnCall Target ip))

(event Custom|AttachToSphereGrav
  (params (Grav :type Actor%20Object%20Reference))
  (bind _ac_nogravcontrol (Variables|Default|GetAC-NoGravControl))
  ;[0.149 0.149 0.149 0.502] Attach and detach devents
  (Components|Tick|SetComponentTickEnabled (Variables|Default|GetAC-NoGravControl) false)
  (Variables|Default|SetisGrav true)
  (bind _output_get (Variables|Default|SetplanetREF Grav))
  (bind _root (Class|BPI-Planet|GetPlanetRoot(Message) _output_get))
  (Transformation|AttachComponentToComponent (Variables|Default|GetOGControlledActor) _root "None" "KeepWorld" "KeepWorld" "KeepWorld" false)
  (Variables|Default|SetPawnMovementControl (Variables|Default|GetAC-SphereGravControl))
  (bind _root_2 (Class|BPI-Planet|GetPlanetRoot(Message) (Variables|Default|GetplanetREF)))
  (CallFunction|OnServerAttachSphere _root_2)
  (Components|Tick|SetComponentTickEnabled (Variables|Default|GetAC-SphereGravControl) true)
  (Variables|/Game/Blueprints/Components/Player/AC-BasePawnMovementControl.AC-BasePawnMovementControl_C|SetxIp _ac_nogravcontrol 0.0)
  (Variables|/Game/Blueprints/Components/Player/AC-BasePawnMovementControl.AC-BasePawnMovementControl_C|SetyIp _ac_nogravcontrol 0.0))

(event Custom|OnServerAttachPlane
  (params (Parent :type Scene%20Component%20Object%20Reference))
  ;[0.149 0.149 0.149 0.502] Attach and detach devents
  (CallFunction|CastAttachPlane Parent))

(event Custom|CastAttachPlane
  (params (Parent :type Scene%20Component%20Object%20Reference))
  ;[0.149 0.149 0.149 0.502] Attach and detach devents
  (if (not (Variables|Default|GetIsLocal))
    (Transformation|AttachComponentToComponent (Variables|Default|GetOGControlledActor) Parent "None" "KeepWorld" "KeepWorld" "KeepWorld" false)
    (Components|Tick|SetComponentTickEnabled (Variables|Default|GetAC-NoGravControl) false)
    (Components|Tick|SetComponentTickEnabled (Variables|Default|GetAC-PlaneGravControl) true)))

(event Custom|CastAttachSphere
  (params (Parent :type Scene%20Component%20Object%20Reference))
  ;[0.149 0.149 0.149 0.502] Attach and detach devents
  (if (not (Variables|Default|GetIsLocal))
    (Transformation|AttachComponentToComponent (Variables|Default|GetOGControlledActor) Parent "None" "KeepWorld" "KeepWorld" "KeepWorld" false)
    (Components|Tick|SetComponentTickEnabled (Variables|Default|GetAC-NoGravControl) false)
    (Components|Tick|SetComponentTickEnabled (Variables|Default|GetAC-SphereGravControl) true)))

(event Custom|OnServerDetach
  ;[0.149 0.149 0.149 0.502] Attach and detach devents
  (CallFunction|CastDetach))

(event Custom|UpdateRelativeLocRotAnims
  (params (Pos :type Vector) (Rot :type Rotator) (curSpeedX :type Float%20%28double-precision%29) (curSpeedY :type Float%20%28double-precision%29) (isInAir :type Boolean))
  (Variables|Cast|SetlocalLocCast Pos)
  (Variables|Cast|SetlocalRotCast Rot)
  (Variables|Cast|SetanimXSpeed curSpeedX)
  (Variables|Cast|SetanimYSpeed curSpeedY)
  (Variables|Cast|SetanimIsInAir isInAir))

(event Custom|PawnActivateGravity
  ;[0.149 0.149 0.149 0.502] Attach and detach devents
  (if (Variables|Default|GetisGrav)
    (CallFunction|DetachfromGravity)
    (else
      (CallFunction|CheckifGravity))))

(event Custom|CastSpawnPawn
  (params (Spawn%20Transform%20Location :type Vector) (Spawn%20Transform%20Rotation :type Rotator))
  (bind _returnvalue (Game|SpawnActorfromClass "/Game/Blueprints/Actors/A-CharacterPawn.A-CharacterPawn_C" (Math|Transform|MakeTransform Spawn%20Transform%20Location Spawn%20Transform%20Rotation "1.000000,1.000000,1.000000") "AdjustIfPossibleButAlwaysSpawn" "MultiplyWithRoot" 0 0))
  (bind _output_get (Variables|Default|SetOGControlledActor _returnvalue))
  (Default|SetControlledPawn (Variables|Default|GetAC-SphereGravControl) _output_get)
  (Components|Tick|SetComponentTickEnabled (Variables|Default|GetAC-NoGravControl) true)
  (Development|PrintString (Utilities|String|Append "CHAR CREATED: " (Utilities|GetDisplayName _output_get))))

(event Custom|AttachToShipGravity
  (params (ship :type A-Base%20Ship%20Object%20Reference))
  (bind _ogcontrolledactor (Variables|Default|GetOGControlledActor))
  (bind _ac_nogravcontrol (Variables|Default|GetAC-NoGravControl))
  (bind _rootcomponent (Variables|/Script/Engine.Actor|GetRootComponent _ogcontrolledactor))
  ;[0.149 0.149 0.149 0.502] Attach and detach devents
  (Components|Tick|SetComponentTickEnabled (Variables|Default|GetAC-NoGravControl) false)
  (Variables|Default|SetisGrav true)
  (bind _output_get (Variables|Default|SetshipActorREF ship))
  (Transformation|AttachComponentToComponent (Variables|Default|GetOGControlledActor) (Variables|/Game/Blueprints/Actors/GravAreas/Ships/A-BaseShip.A-BaseShip_C|GetRoot _output_get) "None" "KeepWorld" "KeepWorld" "KeepWorld" false)
  (Variables|Default|SetPawnMovementControl (Variables|Default|GetAC-PlaneGravControl))
  (CallFunction|OnServerAttachPlane (Variables|/Game/Blueprints/Actors/GravAreas/Ships/A-BaseShip.A-BaseShip_C|GetRoot (Variables|Default|GetshipActorREF)))
  (Components|Tick|SetComponentTickEnabled (Variables|Default|GetAC-PlaneGravControl) true)
  (Variables|/Game/Blueprints/Components/Player/AC-BasePawnMovementControl.AC-BasePawnMovementControl_C|SetxIp _ac_nogravcontrol 0.0)
  (Variables|/Game/Blueprints/Components/Player/AC-BasePawnMovementControl.AC-BasePawnMovementControl_C|SetyIp _ac_nogravcontrol 0.0)
  (Transformation|SetRelativeRotation _rootcomponent (Math|Interpolation|RInterpTo (Variables|/Script/Engine.SceneComponent|GetRelativeRotation _rootcomponent) (Math|Rotator|MakeRotator 0.0 0.0 (.yaw (Variables|/Script/Engine.SceneComponent|GetRelativeRotation _rootcomponent))) 1.0 2.0) false false))

(event Custom|ServerSpawnPawn
  (params (Spawn%20Transform%20Location :type Vector) (Spawn%20Transform%20Rotation :type Rotator))
  (CallFunction|CastSpawnPawn Spawn%20Transform%20Location Spawn%20Transform%20Rotation))

(event Custom|DetachFromGravity
  (bind _ac_planegravcontrol (Variables|Default|GetAC-PlaneGravControl))
  (bind _ogcontrolledactor (Variables|Default|GetOGControlledActor))
  ;[0.149 0.149 0.149 0.502] Attach and detach devents
  (Default|ResetIp _ac_planegravcontrol)
  (Components|Tick|SetComponentTickEnabled _ac_planegravcontrol false)
  (Variables|Default|SetisGrav false)
  (Variables|Default|SetcanDrive false)
  (Transformation|DetachFromActor (Variables|Default|GetOGControlledActor) "KeepWorld" "KeepWorld" "KeepWorld")
  (Variables|Default|SetPawnMovementControl (Variables|Default|GetAC-NoGravControl))
  (Transformation|SetActorRotation _ogcontrolledactor (Math|Interpolation|RInterpTo (Transformation|GetActorRotation _ogcontrolledactor) (Transformation|GetWorldRotation (Variables|Default|GetCamera)) 1.0 3.0))
  (bind _cameraroot (Class|BPI-ActorPawn|GetCameraRoot(Message) (Variables|Default|GetOGControlledActor)))
  (Transformation|SetRelativeRotation _cameraroot (Math|Rotator|MakeRotator 0.0 0.0 0.0) false false)
  (CallFunction|OnServerDetach)
  (Components|Tick|SetComponentTickEnabled (Variables|Default|GetAC-NoGravControl) true)
  (Class|BPI-ActorPawn|SetAnimationVariables(Message) (Variables|Default|GetOGControlledActor) 0.0 0.0 true)
  (Variables|Default|SetshipActorREF 0)
  (Variables|Default|SetplanetREF 0))

(event Custom|OnServerShipHasDriver
  (params (Target :type A-Base%20Ship%20Object%20Reference) (hasDriver :type Boolean))
  ;[0.149 0.149 0.149 0.502] Comment
  (Default|SetHasDriver Target hasDriver))

(event Custom|CheckIfGravity
  ;[0.149 0.149 0.149 0.502] Attach and detach devents
  (bind (_bodycoltop _bodycolend) (Class|BPI-ActorPawn|GetBodyCollisionComponents(Message) (Variables|Default|GetOGControlledActor)))
  (bind (_outhit _returnvalue) (Collision|SphereTraceByChannel (Transformation|GetWorldLocation _bodycoltop) (Transformation|GetWorldLocation _bodycolend) 12.0 "TraceTypeQuery4" false 0 "None"))
  (if _returnvalue
    (if (Utilities|Enum|Equal(Enum) "GravArea" (Utilities|GetObjectName (.HitComponent (Collision|BreakHitResult _outhit))))
      (bind _asa_base_ship (Utilities|Casting|CastToA-BaseShip (Components|GetOwner (.HitComponent (Collision|BreakHitResult _outhit)))))
      (CallFunction|AttachtoShipGravity _asa_base_ship)
      (elif (Utilities|Enum|Equal(Enum) "SphereGravArea" (Utilities|GetObjectName (.HitComponent (Collision|BreakHitResult _outhit))))
        (bind _asa_base_sphere_grav (Utilities|Casting|CastToA-BaseSphereGrav (Components|GetOwner (.HitComponent (Collision|BreakHitResult _outhit)))))
        (CallFunction|AttachtoSphereGrav _asa_base_sphere_grav)))))

(event Input|EnhancedActionEvents|EnhancedInputActionIA_Use
  (params (ActionValue :type Boolean) (ElapsedSeconds :type Float%20%28double-precision%29) (TriggeredSeconds :type Float%20%28double-precision%29) (InputAction :type Input%20Action%20Object%20Reference :default "/Game/Input/Actions/Player/IA_Use.IA_Use"))
  ;[0.149 0.149 0.149 0.502] Pawn input
  (:Started
    (CallFunction|PawnUse)))

(event Input|EnhancedActionEvents|EnhancedInputActionIA_ShipThrust
  (params (ActionValue :type Float%20%28double-precision%29) (ElapsedSeconds :type Float%20%28double-precision%29) (TriggeredSeconds :type Float%20%28double-precision%29) (InputAction :type Input%20Action%20Object%20Reference :default "/Game/Input/Actions/Ship/IA_ShipThrust.IA_ShipThrust"))
  ;[0.15 0.15 0.15 0.5] Ship driving input
  (:Triggered
    (CallFunction|ServerShipThrust (Variables|Default|GetshipActorREF) ActionValue :!label _label))
  (:Canceled
    (goto _label))
  (:Completed
    (goto _label)))

(event Input|EnhancedActionEvents|EnhancedInputActionIA_LookUp
  (params (ActionValue :type Float%20%28double-precision%29) (ElapsedSeconds :type Float%20%28double-precision%29) (TriggeredSeconds :type Float%20%28double-precision%29) (InputAction :type Input%20Action%20Object%20Reference :default "/Game/Input/Actions/Player/IA_LookUp.IA_LookUp"))
  ;[0.149 0.149 0.149 0.502] Pawn input
  (:Triggered
    (Default|LocalLookUp (Variables|Default|GetPawnMovementControl) ActionValue :!label _label))
  (:Canceled
    (goto _label))
  (:Completed
    (goto _label)))

(event Input|EnhancedActionEvents|EnhancedInputActionIA_LookRight
  (params (ActionValue :type Float%20%28double-precision%29) (ElapsedSeconds :type Float%20%28double-precision%29) (TriggeredSeconds :type Float%20%28double-precision%29) (InputAction :type Input%20Action%20Object%20Reference :default "/Game/Input/Actions/Player/IA_LookRight.IA_LookRight"))
  ;[0.149 0.149 0.149 0.502] Pawn input
  (:Triggered
    (Default|LocalRotatePlayer (Variables|Default|GetPawnMovementControl) ActionValue :!label _label))
  (:Canceled
    (goto _label))
  (:Completed
    (goto _label)))

(event Input|EnhancedActionEvents|EnhancedInputActionIA_Jump
  (params (ActionValue :type Boolean) (ElapsedSeconds :type Float%20%28double-precision%29) (TriggeredSeconds :type Float%20%28double-precision%29) (InputAction :type Input%20Action%20Object%20Reference :default "/Game/Input/Actions/Player/IA_Jump.IA_Jump"))
  ;[0.149 0.149 0.149 0.502] Pawn input
  (:Started
    (Default|LocalJump (Variables|Default|GetPawnMovementControl))))

(event Input|EnhancedActionEvents|EnhancedInputActionIA_ActivateGravity
  (params (ActionValue :type Boolean) (ElapsedSeconds :type Float%20%28double-precision%29) (TriggeredSeconds :type Float%20%28double-precision%29) (InputAction :type Input%20Action%20Object%20Reference :default "/Game/Input/Actions/Player/IA_ActivateGravity.IA_ActivateGravity"))
  ;[0.149 0.149 0.149 0.502] Pawn input
  (:Started
    (CallFunction|PawnActivateGravity)))

(event Input|EnhancedActionEvents|EnhancedInputActionIA_Slide
  (params (ActionValue :type Boolean) (ElapsedSeconds :type Float%20%28double-precision%29) (TriggeredSeconds :type Float%20%28double-precision%29) (InputAction :type Input%20Action%20Object%20Reference :default "/Game/Input/Actions/Player/IA_Slide.IA_Slide"))
  ;[0.149 0.149 0.149 0.502] Pawn input
  (:Started
    (Default|LocalSlide (Variables|Default|GetPawnMovementControl) TriggeredSeconds)))

(event Input|EnhancedActionEvents|EnhancedInputActionIA_Crouch
  (params (ActionValue :type Boolean) (ElapsedSeconds :type Float%20%28double-precision%29) (TriggeredSeconds :type Float%20%28double-precision%29) (InputAction :type Input%20Action%20Object%20Reference :default "/Game/Input/Actions/Player/IA_Crouch.IA_Crouch"))
  ;[0.149 0.149 0.149 0.502] Pawn input
  (:Started
    (Default|LocalCrouch (Variables|Default|GetPawnMovementControl) TriggeredSeconds)))

(event Input|EnhancedActionEvents|EnhancedInputActionIA_ShipRoll
  (params (ActionValue :type Float%20%28double-precision%29) (ElapsedSeconds :type Float%20%28double-precision%29) (TriggeredSeconds :type Float%20%28double-precision%29) (InputAction :type Input%20Action%20Object%20Reference :default "/Game/Input/Actions/Ship/IA_ShipRoll.IA_ShipRoll"))
  ;[0.15 0.15 0.15 0.5] Ship driving input
  (:Triggered
    (CallFunction|ServerShipRoll (Variables|Default|GetshipActorREF) ActionValue :!label _label))
  (:Canceled
    (goto _label))
  (:Completed
    (goto _label)))

(event Input|EnhancedActionEvents|EnhancedInputActionIA_MoveForward
  (params (ActionValue :type Float%20%28double-precision%29) (ElapsedSeconds :type Float%20%28double-precision%29) (TriggeredSeconds :type Float%20%28double-precision%29) (InputAction :type Input%20Action%20Object%20Reference :default "/Game/Input/Actions/Player/IA_MoveForward.IA_MoveForward"))
  ;[0.149 0.149 0.149 0.502] Pawn input
  (:Triggered
    (Default|LocalAddMovementX (Variables|Default|GetPawnMovementControl) ActionValue :!label _label))
  (:Canceled
    (goto _label))
  (:Completed
    (goto _label)))

(event Input|EnhancedActionEvents|EnhancedInputActionIA_ShipPull
  (params (ActionValue :type Float%20%28double-precision%29) (ElapsedSeconds :type Float%20%28double-precision%29) (TriggeredSeconds :type Float%20%28double-precision%29) (InputAction :type Input%20Action%20Object%20Reference :default "/Game/Input/Actions/Ship/IA_ShipPull.IA_ShipPull"))
  ;[0.15 0.15 0.15 0.5] Ship driving input
  (:Triggered
    (CallFunction|ServerShipPull (Variables|Default|GetshipActorREF) ActionValue :!label _label))
  (:Canceled
    (goto _label))
  (:Completed
    (goto _label)))

(event Input|EnhancedActionEvents|EnhancedInputActionIA_ShipTurn
  (params (ActionValue :type Float%20%28double-precision%29) (ElapsedSeconds :type Float%20%28double-precision%29) (TriggeredSeconds :type Float%20%28double-precision%29) (InputAction :type Input%20Action%20Object%20Reference :default "/Game/Input/Actions/Ship/IA_ShipTurn.IA_ShipTurn"))
  ;[0.15 0.15 0.15 0.5] Ship driving input
  (:Triggered
    (CallFunction|ServerShipTurn (Variables|Default|GetshipActorREF) ActionValue :!label _label))
  (:Canceled
    (goto _label))
  (:Completed
    (goto _label)))

(event Input|EnhancedActionEvents|EnhancedInputActionIA_MoveRight
  (params (ActionValue :type Float%20%28double-precision%29) (ElapsedSeconds :type Float%20%28double-precision%29) (TriggeredSeconds :type Float%20%28double-precision%29) (InputAction :type Input%20Action%20Object%20Reference :default "/Game/Input/Actions/Player/IA_MoveRight.IA_MoveRight"))
  ;[0.149 0.149 0.149 0.502] Pawn input
  (:Triggered
    (Default|LocalAddMovementY (Variables|Default|GetPawnMovementControl) ActionValue :!label _label))
  (:Canceled
    (goto _label))
  (:Completed
    (goto _label)))

(event EventBeginPlay
  (|CallParentFunction)
  (bind _aspc_main (Utilities|Casting|CastToPC-Main (Game|GetPlayerController 0)))
  (Variables|Default|Setpc _aspc_main)
  (Utilities|FlowControl|Delay 1.0)
  (if (Pawn|IsLocallyControlled)
    (Variables|Default|SetIsLocal true)
    (else
      (Variables|Default|SetIsLocal false))))

(event EventSetGlobalLocationRotation
  (params (NewLocation :type Vector :default "0, 0, 0") (NewRotation :type Rotator :default "0, 0, 0"))
  (Variables|Cast|SetglobalLocCast NewLocation)
  (Variables|Cast|SetglobalRotCast NewRotation))

(event EventCallDetachfromGravity
  (CallFunction|DetachfromGravity))

(event EventSetCanDrive
  (params (CanDrive :type Boolean))
  (Variables|Default|SetcanDrive CanDrive))

(event EventSetRelativeLocationRotationAnimation
  (params (Pos :type Vector :default "0, 0, 0") (Rot :type Rotator :default "0, 0, 0") (CurSpeedX :type Float%20%28double-precision%29) (CurSpeedY :type Float%20%28double-precision%29) (IsInAir :type Boolean))
  (CallFunction|UpdateRelativeLocRotAnims Pos Rot CurSpeedX CurSpeedY IsInAir))

(fn ConstructionScript
  (|CallParentFunction))

(fn GetUpdatedGlobalLocRot
  (return (Variables|Cast|GetglobalLocCast) (Variables|Cast|GetglobalRotCast)))

(fn GetUpdatedRelativeLocRotAnims
  (return (Variables|Cast|GetlocalLocCast) (Variables|Cast|GetlocalRotCast) (Variables|Cast|GetanimXSpeed) (Variables|Cast|GetanimYSpeed) (Variables|Cast|GetanimIsInAir)))

(fn GetAttachedPlanet
  (return (Variables|Default|GetplanetREF)))

(fn GetAttachedShip
  (return (Variables|Default|GetshipActorREF)))

(fn GetControlledActor
  (return (Variables|Default|GetOGControlledActor)))

(fn GetGlobalLocationRotation
  (return (Variables|Cast|GetglobalLocCast) (Variables|Cast|GetglobalRotCast)))

(fn GetIsLocal
  (return (Variables|Default|GetIsLocal)))

(fn GetRelativeLocationRotationAnimation
  (return (Variables|Cast|GetlocalLocCast) (Variables|Cast|GetlocalRotCast) (Variables|Cast|GetanimXSpeed) (Variables|Cast|GetanimYSpeed) (Variables|Cast|GetanimIsInAir)))